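; BP_GoToToiletEvent is a quest event that sends a passenger to the toilet and back to their seat.
; On EnterEvent it casts the participant to FABasePassenger and finds a BP_ToiletWaypoint with GetActorOfClass.
; It queues stand, move to waypoint, move to assigned seat and sit actions on the passenger's ActionExecutorComponent, then executes them.
; The sequence has no wait action at the toilet.
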(event EventEnterEvent
  (params (Context :type Dlg%20Context%20Object%20Reference) (Participant :type Object%20Object%20Reference))
  (bind _asfabase_passenger (Utilities|Casting|CastToFABasePassenger Participant))
  (bind _returnvalue (Actor|GetActorOfClass "/Game/SpaceShip/Toilet/BP_ToiletWaypoint.BP_ToiletWaypoint_C"))
  (Class|ActionExecutorComponent|SetActions (Variables|/Script/FlightAttendantSim.FABaseCharacter|GetActionExecutorComponent _asfabase_passenger) (Utilities|Array|MakeArray (Class|CharacterStandAction|CreateCharacterStandAction (Variables|/Script/FlightAttendantSim.FABaseCharacter|GetActionExecutorComponent _asfabase_passenger)) (Class|CharacterMoveAction|CreateCharacterMoveAction (Transformation|GetActorLocation _returnvalue) (Variables|/Script/FlightAttendantSim.FABaseCharacter|GetActionExecutorComponent _asfabase_passenger)) (Class|CharacterMoveAction|CreateCharacterMoveAction (Transformation|GetWorldLocation (Variables|/Script/FlightAttendantSim.Seat|GetMoveToLocation (Variables|/Script/FlightAttendantSim.FABasePassenger|GetAssignedPassengerSeat _asfabase_passenger))) (Variables|/Script/FlightAttendantSim.FABaseCharacter|GetActionExecutorComponent _asfabase_passenger)) (Class|CharacterSitAction|CreateCharacterSitAction (Variables|/Script/FlightAttendantSim.FABasePassenger|GetAssignedPassengerSeat _asfabase_passenger) (Variables|/Script/FlightAttendantSim.FABaseCharacter|GetActionExecutorComponent _asfabase_passenger))))
  (Class|ActionExecutorComponent|ExecuteActions (Variables|/Script/FlightAttendantSim.FABaseCharacter|GetActionExecutorComponent _asfabase_passenger)))