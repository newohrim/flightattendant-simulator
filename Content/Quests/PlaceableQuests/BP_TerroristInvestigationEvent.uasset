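; Placeable quest event that resolves the terrorist investigation in Q_AlphaQuest1 based on the chosen passenger seat.
; On EnterEvent it matches the seat title among the SpacePlane's seats and takes the assigned passenger.
; The passenger's position in AssignedPassengers picks the outcome passed to TerroristInvestigationEnd, with separate results for last, second-to-last and any other.
; A "None" seat choice ends the investigation with its own outcome.
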(event EventEnterEvent
  (params (Context :type Dlg%20Context%20Object%20Reference) (Participant :type Object%20Object%20Reference))
  (bind _asfagame_mode (Utilities|Casting|CastToFAGameMode (Game|GetGameMode)))
  (bind _asq_alpha_quest_1 (Utilities|Casting|CastToQ_AlphaQuest1 (Class|FAGameMode|GetQuestfromClass _asfagame_mode (Variables|Default|GetQuestClass))))
  (if (Utilities|Enum|Equal(Enum) (Variables|Default|GetChoosenSeat) "None")
    (Default|TerroristInvestigationEnd _asq_alpha_quest_1 "NewEnumerator3")
    (else
      (bind _array_element (Utilities|Array|ForEachLoopwithBreak (Variables|/Script/FlightAttendantSim.SpacePlaneComponent|GetPassengerSeats (Variables|/Script/FlightAttendantSim.FAGameMode|GetSpacePlane _asfagame_mode)) :!label _label)
        (:LoopBody
          (if (Utilities|Enum|Equal(Enum) (Variables|/Script/FlightAttendantSim.PassengerSeat|GetSeatTitle _array_element) (Variables|Default|GetChoosenSeat))
            (bind _asfabase_passenger (Utilities|Casting|CastToFABasePassenger (Variables|/Script/FlightAttendantSim.Seat|GetAssignedCharacter _array_element)))
            (Default|TerroristInvestigationEnd _asq_alpha_quest_1 (select (== (Utilities|Array|FindItem (Variables|/Script/FlightAttendantSim.SpacePlaneComponent|GetAssignedPassengers (Variables|/Script/FlightAttendantSim.FAGameMode|GetSpacePlane _asfagame_mode)) _asfabase_passenger) (- (Utilities|Array|Length (Variables|/Script/FlightAttendantSim.SpacePlaneComponent|GetAssignedPassengers (Variables|/Script/FlightAttendantSim.FAGameMode|GetSpacePlane _asfagame_mode))) 1)) "NewEnumerator0" (select (== (Utilities|Array|FindItem (Variables|/Script/FlightAttendantSim.SpacePlaneComponent|GetAssignedPassengers (Variables|/Script/FlightAttendantSim.FAGameMode|GetSpacePlane _asfagame_mode)) _asfabase_passenger) (- (- (Utilities|Array|Length (Variables|/Script/FlightAttendantSim.SpacePlaneComponent|GetAssignedPassengers (Variables|/Script/FlightAttendantSim.FAGameMode|GetSpacePlane _asfagame_mode))) 1) 1)) "NewEnumerator1" "NewEnumerator2")))
            (goto _label Break)))))))