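; Quest transition event that randomly picks a terrorist and a fake terrorist from the space plane's assigned passengers.
; When at least two passengers exist, it swaps random entries into the last two array slots, a partial shuffle that guarantees distinct picks.
; Those two receive the terrorist and fake terrorist dialogues on their DialogueComponents, and all other passengers receive the default dialogue.
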(event EventExecute
  (bind _asfagame_mode (Utilities|Casting|CastToFAGameMode (Class|Quest|GetGameModeHelperStatic self)))
  (if (>= (Utilities|Array|Length (Variables|/Script/FlightAttendantSim.SpacePlaneComponent|GetAssignedPassengers (Variables|/Script/FlightAttendantSim.FAGameMode|GetSpacePlane _asfagame_mode))) 2)
    (Utilities|Array|Swap (Variables|/Script/FlightAttendantSim.SpacePlaneComponent|GetAssignedPassengers (Variables|/Script/FlightAttendantSim.FAGameMode|GetSpacePlane _asfagame_mode)) (Math|Random|RandomInteger (Utilities|Array|Length (Variables|/Script/FlightAttendantSim.SpacePlaneComponent|GetAssignedPassengers (Variables|/Script/FlightAttendantSim.FAGameMode|GetSpacePlane _asfagame_mode)))) (- (Utilities|Array|Length (Variables|/Script/FlightAttendantSim.SpacePlaneComponent|GetAssignedPassengers (Variables|/Script/FlightAttendantSim.FAGameMode|GetSpacePlane _asfagame_mode))) 1))
    (Utilities|Array|Swap (Variables|/Script/FlightAttendantSim.SpacePlaneComponent|GetAssignedPassengers (Variables|/Script/FlightAttendantSim.FAGameMode|GetSpacePlane _asfagame_mode)) (Math|Random|RandomInteger (- (Utilities|Array|Length (Variables|/Script/FlightAttendantSim.SpacePlaneComponent|GetAssignedPassengers (Variables|/Script/FlightAttendantSim.FAGameMode|GetSpacePlane _asfagame_mode))) 1)) (- (- (Utilities|Array|Length (Variables|/Script/FlightAttendantSim.SpacePlaneComponent|GetAssignedPassengers (Variables|/Script/FlightAttendantSim.FAGameMode|GetSpacePlane _asfagame_mode))) 1) 1))
    (for _index (range 0 (- (- (- (Utilities|Array|Length (Variables|/Script/FlightAttendantSim.SpacePlaneComponent|GetAssignedPassengers (Variables|/Script/FlightAttendantSim.FAGameMode|GetSpacePlane _asfagame_mode))) 1) 1) 1))
      (Variables|/Script/FlightAttendantSim.DialogueComponent|SetAssignedDialogue (Variables|/Script/FlightAttendantSim.FABaseCharacter|GetDialogueComponent (Utilities|Array|Get(acopy) (Variables|/Script/FlightAttendantSim.SpacePlaneComponent|GetAssignedPassengers (Variables|/Script/FlightAttendantSim.FAGameMode|GetSpacePlane _asfagame_mode)) _index)) (Variables|Default|GetDefaultDialogue)))
    (Variables|/Script/FlightAttendantSim.DialogueComponent|SetAssignedDialogue (Variables|/Script/FlightAttendantSim.FABaseCharacter|GetDialogueComponent (Utilities|Array|Get(acopy) (Variables|/Script/FlightAttendantSim.SpacePlaneComponent|GetAssignedPassengers (Variables|/Script/FlightAttendantSim.FAGameMode|GetSpacePlane _asfagame_mode)) (- (Utilities|Array|Length (Variables|/Script/FlightAttendantSim.SpacePlaneComponent|GetAssignedPassengers (Variables|/Script/FlightAttendantSim.FAGameMode|GetSpacePlane _asfagame_mode))) 1))) (Variables|Default|GetTerroristDialogue))
    (Variables|/Script/FlightAttendantSim.DialogueComponent|SetAssignedDialogue (Variables|/Script/FlightAttendantSim.FABaseCharacter|GetDialogueComponent (Utilities|Array|Get(acopy) (Variables|/Script/FlightAttendantSim.SpacePlaneComponent|GetAssignedPassengers (Variables|/Script/FlightAttendantSim.FAGameMode|GetSpacePlane _asfagame_mode)) (- (- (Utilities|Array|Length (Variables|/Script/FlightAttendantSim.SpacePlaneComponent|GetAssignedPassengers (Variables|/Script/FlightAttendantSim.FAGameMode|GetSpacePlane _asfagame_mode))) 1) 1))) (Variables|Default|GetFakeTerroristDialogue))))