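; BP_Pawn is the briefing demo's pawn, which forwards player input to a BriefingComponent.
; Three FigureGoodZone input actions each call ExecuteTest with their zone index on press, and releasing R calls SwapRows.
; BeginPlay records the current wall-clock time of day in seconds as StartTime, which this graph does not read again.
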(event EventBeginPlay
  (Variables|Default|SetStartTime (Math|Timespan|GetTotalSeconds (TimeOfDay|GetTimeOfDay (Math|DateTime|Now) :!class /Script/Engine.KismetMathLibrary))))

(event Collision|EventActorBeginOverlap
  (params (OtherActor :type Actor%20Object%20Reference)))

(event EventTick
  (params (DeltaSeconds :type Float%20%28single-precision%29)))

(event Input|ActionEvents|InputActionFigureGoodZone1
  (params (Key :type Key%20Structure :default "None"))
  (:Pressed
    (Default|ExecuteTest (Variables|Default|GetBriefingComponent))))

(event Input|ActionEvents|InputActionFigureGoodZone2
  (params (Key :type Key%20Structure :default "None"))
  (:Pressed
    (Default|ExecuteTest (Variables|Default|GetBriefingComponent) 1)))

(event Input|ActionEvents|InputActionFigureGoodZone3
  (params (Key :type Key%20Structure :default "None"))
  (:Pressed
    (Default|ExecuteTest (Variables|Default|GetBriefingComponent) 2)))

(event Input|KeyboardEvents|R
  (params (Key :type Key%20Structure :default "None"))
  (:Released
    (Default|SwapRows (Variables|Default|GetBriefingComponent))))

(fn ConstructionScript)