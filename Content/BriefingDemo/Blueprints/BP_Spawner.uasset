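; BP_Spawner is an actor that repeatedly spawns random figures at its own transform in the briefing demo.
; On BeginPlay it caches the pawn's BP_BriefingComponent and the game mode's FigureBuffer class list.
; A randomized Delay on Tick acts as the spawn timer, checking the component's shutdown condition after each wait.
; When that condition holds it calls Shutdown on the component, otherwise it spawns another figure regardless of collision.
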(event EventBeginPlay
  (bind _returnvalue (Actor|GetActorOfClass "/Game/BriefingDemo/Blueprints/BP_Pawn.BP_Pawn_C"))
  (Variables|Default|SetBriefingComponent (Actor|GetComponentbyClass _returnvalue "/Game/BriefingDemo/Blueprints/BP_BriefingComponent.BP_BriefingComponent_C"))
  (bind _asbp_fabase_game_mode (Utilities|Casting|CastToBP_FABaseGameMode (Game|GetGameMode)))
  (Variables|Default|SetFigureClasses (Variables|/Game/DocumentsCheck/BP_FABaseGameMode.BP_FABaseGameMode_C|GetFigureBuffer _asbp_fabase_game_mode)))

(event Collision|EventActorBeginOverlap
  (params (OtherActor :type Actor%20Object%20Reference)))

(event EventTick
  (params (DeltaSeconds :type Float%20%28single-precision%29))
  (Utilities|FlowControl|Delay (Math|Random|RandomFloatinRange 0.5 3.0))
  (if (Default|CheckShutdownCondition (Variables|Default|GetBriefingComponent))
    (Default|Shutdown (Variables|Default|GetBriefingComponent))
    (else
      (Game|SpawnActorfromClass (.OutItem (Utilities|Array|Random (Variables|Default|GetFigureClasses))) (Transformation|GetActorTransform) "AlwaysSpawn" 0 0))))

(fn ConstructionScript)