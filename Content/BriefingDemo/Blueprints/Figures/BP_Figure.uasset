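; BP_Figure is a moving actor that costs the player health when it reaches a death zone.
; Each tick it moves along world X, scaled by Speed and a fixed cosine factor; its Z term uses a zero-degree sine, so height stays constant.
; On overlapping a BP_DeathZone, it subtracts one HP from player 0's BP_Pawn and destroys itself.
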(event EventBeginPlay)

(event Collision|EventActorBeginOverlap
  (params (OtherActor :type Actor%20Object%20Reference))
  (Utilities|Casting|CastToBP_DeathZone OtherActor)
  (bind _asbp_pawn (Utilities|Casting|CastToBP_Pawn (Game|Player|GetPlayerPawn 0)))
  (Variables|/Game/BriefingDemo/Blueprints/BP_Pawn.BP_Pawn_C|SetHP _asbp_pawn (- (Variables|/Game/BriefingDemo/Blueprints/BP_Pawn.BP_Pawn_C|GetHP _asbp_pawn) 1.0))
  (Actor|DestroyActor))

(event EventTick
  (params (DeltaSeconds :type Float%20%28single-precision%29))
  (bind _returnvalue (Transformation|GetActorLocation))
  (Transformation|SetActorLocation (Math|Vector|MakeVector (+ (* DeltaSeconds (Variables|Default|GetSpeed) (Math|Trig|Cos(Degrees) 1e+01)) (.x _returnvalue)) (.y _returnvalue) (- (.z _returnvalue) (* DeltaSeconds (Math|Trig|Sin(Degrees) 0.0) (Variables|Default|GetSpeed)))) false false))

(fn ConstructionScript)