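; BP_BriefingComponent runs the logic of a briefing phase in which figures in zones are tested against each zone's expected class.
; ExecuteTest destroys the first matching figure in the chosen zone and reports a good or bad hit to the game mode.
; StartPhase swaps two zones' classes once after a random delay, mirroring it in W_BriefingUI.
; Shutdown clears spawners, notifies the game mode and destroys its owner.
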(event Custom|StartPhase
  (Utilities|FlowControl|Delay (Math|Random|RandomFloatinRange 7.5 15.0))
  (CallFunction|SwapRows))

(event EventBeginPlay
  (bind _asbp_fabase_game_mode (Utilities|Casting|CastToBP_FABaseGameMode (Game|GetGameMode)))
  (Variables|Default|SetGameMode _asbp_fabase_game_mode)
  (bind _asbp_fabase_game_state (Utilities|Casting|CastToBP_FABaseGameState (Game|GetGameState)))
  (Variables|Default|SetGameState _asbp_fabase_game_state))

(event EventTick
  (params (DeltaSeconds :type Float%20%28single-precision%29)))

(fn GoodHit
  (Default|BriefingGoodHit (Variables|Default|GetGameMode)))

(fn BadHit
  (Default|BriefingBadHit (Variables|Default|GetGameMode)))

(fn CheckifGoodHit
  (params (GoodZone :type BP%20Good%20Zone%20Object%20Reference))
  (bind _output_get (LocalVariables|SetClassIndex (.Value (Utilities|Map|Find (Variables|Default|GetClassToIndexMap) (Variables|/Game/BriefingDemo/Blueprints/BP_GoodZone.BP_GoodZone_C|GetFigureClass GoodZone)))))
  (bind (_array_element _array_index) (Utilities|Array|ForEachLoopwithBreak (Variables|/Game/BriefingDemo/Blueprints/BP_GoodZone.BP_GoodZone_C|Getobjects GoodZone))
    (:LoopBody
      (LocalVariables|SetCurrentFigure _array_element)
      (switch int _output_get
        (:Default
          _)
        (:0
          (Utilities|Casting|CastToBP_FigureCube _array_element)
          (Utilities|Array|RemoveIndex (Variables|/Game/BriefingDemo/Blueprints/BP_GoodZone.BP_GoodZone_C|Getobjects GoodZone) _array_index :!label _label)
          (Actor|DestroyActor (LocalVariables|GetCurrentFigure))
          (return true))
        (:1
          (Utilities|Casting|CastToBP_FigureSphere _array_element)
          (goto _label))
        (:2
          (Utilities|Casting|CastToBP_FigureTriangle _array_element)
          (goto _label))))
    (:Completed
      _))
  (return false))

(fn ExecuteTest
  (params (ZoneIndex :type Integer))
  (if (CallFunction|CheckifGoodHit (Utilities|Array|Get(acopy) (Variables|Briefing|GetGoodZones) ZoneIndex))
    (CallFunction|GoodHit)
    (else
      (CallFunction|BadHit))))

(fn Shutdown
  (for _array_element (Variables|Briefing|GetFigureSpawners)
    (Actor|DestroyActor _array_element))
  (Utilities|Array|Clear (Variables|Briefing|GetFigureSpawners))
  (Default|BriefingPhaseCompleted (Variables|Default|GetGameMode))
  (Actor|DestroyActor (Components|GetOwner)))

(fn CheckShutdownCondition
  (bind _gamestate (Variables|Default|GetGameState))
  (return (>= (Variables|/Game/DocumentsCheck/BP_FABaseGameState.BP_FABaseGameState_C|GetGoodFigures _gamestate) (Variables|/Game/DocumentsCheck/BP_FABaseGameState.BP_FABaseGameState_C|GetFiguresToCompletePhase _gamestate))))

(fn SwapRows
  (bind _goodzones (Variables|Briefing|GetGoodZones))
  (bind _output_get (LocalVariables|SetN (Utilities|Array|Length (Variables|Briefing|GetGoodZones))))
  (bind _output_get_2 (LocalVariables|SetRandIndex (Math|Random|RandomInteger _output_get)))
  (bind _output_get_3 (LocalVariables|SetIndexA (CallFunction|TrueModulo (+ _output_get_2 1) (LocalVariables|GetN))))
  (bind _output_get_4 (LocalVariables|SetIndexB (CallFunction|TrueModulo (- _output_get_2 1) (LocalVariables|GetN))))
  (Development|PrintString (Utilities|String|ToString(Integer) _output_get_3))
  (Development|PrintString (Utilities|String|ToString(Integer) _output_get_4))
  (bind _output_get_5 (LocalVariables|SetTempClass (Variables|/Game/BriefingDemo/Blueprints/BP_GoodZone.BP_GoodZone_C|GetFigureClass (Utilities|Array|Get(acopy) _goodzones _output_get_3))))
  (Variables|/Game/BriefingDemo/Blueprints/BP_GoodZone.BP_GoodZone_C|SetFigureClass (Utilities|Array|Get(acopy) _goodzones _output_get_3) (Variables|/Game/BriefingDemo/Blueprints/BP_GoodZone.BP_GoodZone_C|GetFigureClass (Utilities|Array|Get(acopy) _goodzones (LocalVariables|GetIndexB))))
  (Variables|/Game/BriefingDemo/Blueprints/BP_GoodZone.BP_GoodZone_C|SetFigureClass (Utilities|Array|Get(acopy) _goodzones (LocalVariables|GetIndexB)) _output_get_5)
  (bind _foundwidgets (Widget|GetAllWidgetsOfClass "/Game/BriefingDemo/Blueprints/UI/W_BriefingUI.W_BriefingUI_C" true))
  (Default|SwapRows (Utilities|Array|Get(acopy) _foundwidgets) (LocalVariables|GetIndexA) (LocalVariables|GetIndexB)))

(fn TrueModulo
  (params (A :type Integer) (B :type Integer))
  (bind _returnvalue (Math|Integer|%(Integer) A B))
  (return (Math|Integer|SelectInt _returnvalue (+ _returnvalue B) (>= _returnvalue 0))))