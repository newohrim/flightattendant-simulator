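; BP_GoodZone is a zone actor in the briefing demo that tracks the BP_Figure actors overlapping it in an Objects array.
; When a tracked figure leaves and its class matches FigureClass, it calls BriefingBadHit on BP_FABaseGameMode.
; DestroyFirstFigure destroys the oldest entry, shifts the array down and shrinks it, or clears it if the new first entry is invalid.
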(event EventBeginPlay)

(event Collision|EventActorBeginOverlap
  (params (OtherActor :type Actor%20Object%20Reference))
  (bind _asbp_figure (Utilities|Casting|CastToBP_Figure OtherActor))
  (Utilities|Array|Add (Variables|Default|Getobjects) _asbp_figure))

(event EventTick
  (params (DeltaSeconds :type Float%20%28single-precision%29)))

(event Collision|EventActorEndOverlap
  (params (OtherActor :type Actor%20Object%20Reference))
  (bind _asbp_figure (Utilities|Casting|CastToBP_Figure OtherActor))
  (bind _returnvalue (Utilities|Array|RemoveItem (Variables|Default|Getobjects) _asbp_figure))
  (if _returnvalue
    (if (== (Utilities|GetClass _asbp_figure) (Variables|Default|GetFigureClass))
      (bind _asbp_fabase_game_mode (Utilities|Casting|CastToBP_FABaseGameMode (Game|GetGameMode)))
      (Default|BriefingBadHit _asbp_fabase_game_mode))))

(fn ConstructionScript)

(fn DestroyFirstFigure
  (bind _objects (Variables|Default|Getobjects))
  (bind _objects_2 (Variables|Default|Getobjects))
  (if (> (Utilities|Array|Length (Variables|Default|Getobjects)) 0)
    (Actor|DestroyActor (Utilities|Array|Get(acopy) (Variables|Default|Getobjects)))
    (for _index (range 0 (- (Utilities|Array|Length (Variables|Default|Getobjects)) 2))
      (Utilities|Array|SetArrayElem _objects _index (Utilities|Array|Get(acopy) _objects (+ _index 1))))
    (Utilities|IsValid (Utilities|Array|Get(acopy) _objects)
      (:Is%20Valid
        (Utilities|Array|Resize _objects_2 (- (Utilities|Array|Length _objects_2) 1)))
      (:Is%20Not%20Valid
        (Utilities|Array|Clear _objects_2)))))