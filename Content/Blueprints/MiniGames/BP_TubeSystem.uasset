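; BP_TubeSystem is a minigame actor with custom events for opening and closing box doors, though all four rotate only Door1.
; Each event loops through a 0.01-second Delay, stepping world roll one degree until the wrapped angle passes its 150 or 180 degree limit.
; Only CloseBoxRight increases roll; the other three decrease it, and OpenBoxRight prints the final rotation.
; Nothing in this Blueprint calls these events.
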(event Custom|OpenBoxLeft
  (bind _door1 (Variables|Default|GetDoor1))
  (bind _returnvalue (Transformation|GetWorldRotation _door1))
  (if (< (Math|Float|%(Float) (+ (.roll (Transformation|GetWorldRotation (Variables|Default|GetDoor1))) 3.6e+02) 3.6e+02) 1.8e+02) :!label _label
    (Transformation|SetWorldRotation _door1 (Math|Rotator|MakeRotator (- (.roll _returnvalue) 1.0) (.pitch _returnvalue) (.yaw _returnvalue)) false false)
    (Utilities|FlowControl|Delay 0.01)
    (goto _label)))

(event Custom|CloseBoxLeft
  (bind _door1 (Variables|Default|GetDoor1))
  (bind _returnvalue (Transformation|GetWorldRotation _door1))
  (if (> (Math|Float|%(Float) (+ (.roll (Transformation|GetWorldRotation (Variables|Default|GetDoor1))) 3.6e+02) 3.6e+02) 1.5e+02) :!label _label
    (Transformation|SetWorldRotation _door1 (Math|Rotator|MakeRotator (+ (.roll _returnvalue) -1.0) (.pitch _returnvalue) (.yaw _returnvalue)) false false)
    (Utilities|FlowControl|Delay 0.01)
    (goto _label)))

(event Custom|OpenBoxRight
  (bind _door1 (Variables|Default|GetDoor1))
  (bind _door1_2 (Variables|Default|GetDoor1))
  (bind _returnvalue (Transformation|GetWorldRotation _door1_2))
  (if (> (Math|Float|%(Float) (+ (.roll (Transformation|GetWorldRotation _door1)) 3.6e+02) 3.6e+02) 1.5e+02) :!label _label
    (Transformation|SetWorldRotation _door1_2 (Math|Rotator|MakeRotator (- (.roll _returnvalue) 1.0) (.pitch _returnvalue) (.yaw _returnvalue)) false false)
    (Utilities|FlowControl|Delay 0.01)
    (goto _label)
    (else
      (Development|PrintString (Utilities|String|ToString(Rotator) (Transformation|GetWorldRotation _door1))))))

(event Custom|CloseBoxRight
  (bind _door1 (Variables|Default|GetDoor1))
  (bind _returnvalue (Transformation|GetWorldRotation _door1))
  (if (< (Math|Float|%(Float) (+ (.roll (Transformation|GetWorldRotation (Variables|Default|GetDoor1))) 3.6e+02) 3.6e+02) 1.5e+02) :!label _label
    (Transformation|SetWorldRotation _door1 (Math|Rotator|MakeRotator (+ (.roll _returnvalue) 1.0) (.pitch _returnvalue) (.yaw _returnvalue)) false false)
    (Utilities|FlowControl|Delay 0.01)
    (goto _label)))

(event EventBeginPlay)

(event Collision|EventActorBeginOverlap
  (params (OtherActor :type Actor%20Object%20Reference)))

(event EventTick
  (params (DeltaSeconds :type Float%20%28single-precision%29)))

(fn ConstructionScript)