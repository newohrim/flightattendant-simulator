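; Tube piece for a mini-game that animates a quarter turn of its root component each time Rotate90 is called.
; BeginPlay caches the relative rotation, then Rotate90 steps pitch down one degree per short Delay in a counted loop, wrapping it with modulo 360.
; An IsRotating flag ignores calls made mid-turn.
; Debug strings print during and after each turn, and the Check event is an empty stub.
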(event Custom|Rotate90
  (if (not (Variables|Default|GetisRotating))
    (Variables|Default|SetisRotating true)
    (bind _output_get (Variables|Default|Setcounter 0))
    (if (< _output_get 90) :!label _label
      (bind _output_get_2 (Variables|Default|SetTempRotation (Math|Rotator|MakeRotator (.Roll (Math|Rotator|BreakRotator (Variables|Default|GetTempRotation))) (Math|Conversions|ToFloat(Integer) (Math|Integer|%(Integer) (+ (Math|Float|Round (+ (.Pitch (Math|Rotator|BreakRotator (Variables|Default|GetTempRotation))) -1.0)) 360) 360)) (.Yaw (Math|Rotator|BreakRotator (Variables|Default|GetTempRotation))))))
      (Development|PrintString (Utilities|String|Append (Utilities|String|ToString(Rotator) _output_get_2) "////" (Utilities|String|ToString(Float) 0.0)) true true "(R=1.000000,G=0.079394,B=0.000000,A=1.000000)" 2e+02)
      (Transformation|SetRelativeRotation (Variables|Default|GetDefaultSceneRoot) _output_get_2 false false)
      (Variables|Default|Setcounter (+ (Variables|Default|Getcounter) 1))
      (Utilities|FlowControl|Delay 0.01)
      (goto _label)
      (else
        (Variables|Default|SetisRotating false)
        (Development|PrintString "Hello")))))

(event Custom|Check)

(event EventBeginPlay
  (Variables|Default|SetTempRotation (Variables|/Script/Engine.SceneComponent|GetRelativeRotation (Variables|Default|GetDefaultSceneRoot))))

(fn ConstructionScript)