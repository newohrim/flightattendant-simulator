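; BP_WireSystem is a minigame Blueprint that, as scripted so far, only opens and closes a box door, with no wire logic.
; OpenBox and CloseBox events step Door1's pitch one degree at a time through self-looping short Delays, swinging between level and roughly -90 degrees.
; Each loop stops by testing floored pitch wrapped into 0–360, then prints a debug message.
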(event Custom|OpenBox
  (bind _door1 (Variables|Default|GetDoor1))
  (bind _door1_2 (Variables|Default|GetDoor1))
  (bind _relativerotation (Variables|/Script/Engine.SceneComponent|GetRelativeRotation _door1_2))
  (bind _relativerotation_2 (Variables|/Script/Engine.SceneComponent|GetRelativeRotation _door1))
  (bind _returnvalue (Math|Float|Floor (.pitch _relativerotation_2)))
  (bind _returnvalue_2 (+ _returnvalue 360))
  (bind _returnvalue_3 (Math|Integer|%(Integer) _returnvalue_2 360))
  (if (or (== _returnvalue_3 0) (and (< _returnvalue_3 360) (> _returnvalue_3 270))) :!label _label
    (Transformation|SetRelativeRotation (Variables|Default|GetDoor1) (Math|Rotator|MakeRotator (.roll _relativerotation) (- (.pitch _relativerotation) 1.0) (.yaw _relativerotation)) false false)
    (Utilities|FlowControl|Delay 0.01)
    (goto _label)
    (else
      (Development|PrintString "Opened"))))

(event Custom|CloseBox
  (bind _door1 (Variables|Default|GetDoor1))
  (bind _door1_2 (Variables|Default|GetDoor1))
  (bind _relativerotation (Variables|/Script/Engine.SceneComponent|GetRelativeRotation _door1_2))
  (bind _relativerotation_2 (Variables|/Script/Engine.SceneComponent|GetRelativeRotation _door1))
  (bind _returnvalue (Math|Float|Floor (.pitch _relativerotation_2)))
  (bind _returnvalue_2 (+ _returnvalue 360))
  (bind _returnvalue_3 (Math|Integer|%(Integer) _returnvalue_2 360))
  (if (and (< _returnvalue_3 360) (>= _returnvalue_3 270)) :!label _label
    (Transformation|SetRelativeRotation (Variables|Default|GetDoor1) (Math|Rotator|MakeRotator (.roll _relativerotation) (+ (.pitch _relativerotation) 1.0) (.yaw _relativerotation)) false false)
    (Utilities|FlowControl|Delay 0.01)
    (goto _label)
    (else
      (Development|PrintString "Closed"))))

(event EventBeginPlay)

(event Collision|EventActorBeginOverlap
  (params (OtherActor :type Actor%20Object%20Reference)))

(event EventTick
  (params (DeltaSeconds :type Float%20%28single-precision%29)))

(fn ConstructionScript)