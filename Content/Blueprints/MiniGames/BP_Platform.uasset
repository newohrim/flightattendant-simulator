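; BP_Platform is a moving platform for the minigames that shuttles a cube between its Start and End component positions.
; From BeginPlay, a latent MoveComponentTo loop moves Cube1 over a fixed duration per leg, flipping ToEnd to alternate direction.
; The Moving flag is checked before each leg, so the loop ends for good once it reads false.
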(event EventBeginPlay
  (bind _cube1 (Variables|Default|GetCube1))
  (Utilities|FlowControl|Sequence
    (:then_0
      (if (Variables|Default|Getmoving) :!label _label
        (if (Variables|Default|GettoEnd)
          (Components|MoveComponentTo _cube1 (Variables|/Script/Engine.SceneComponent|GetRelativeLocation (Variables|Default|Getend)) "0, 0, 0" false false 2.0 false)
          (Variables|Default|SettoEnd false)
          (goto _label)
          (else
            (Components|MoveComponentTo _cube1 (Variables|/Script/Engine.SceneComponent|GetRelativeLocation (Variables|Default|Getstart)) "0, 0, 0" false false 2.0 false)
            (Variables|Default|SettoEnd true)
            (goto _label)))))))

(event Collision|EventActorBeginOverlap
  (params (OtherActor :type Actor%20Object%20Reference)))

(event EventTick
  (params (DeltaSeconds :type Float%20%28single-precision%29)))

(fn ConstructionScript)