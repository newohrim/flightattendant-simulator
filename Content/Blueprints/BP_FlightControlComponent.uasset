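; BP_FlightControlComponent handles what changes when a flight starts and ends.
; It toggles the warp cone material parameter, notifies the weather radar on the control table display, and disables saving in the pause menu during flight.
; On flight start it also gives assigned space plane passengers a random chance, set by MakeOrderRate, to place an order, then initializes their status widget with it.
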(event Custom|MakeOrders
  (bind _asfagame_mode (Utilities|Casting|CastToFAGameMode (Game|GetGameMode)))
  (for _array_element (Variables|/Script/FlightAttendantSim.SpacePlaneComponent|GetAssignedPassengers (Variables|/Script/FlightAttendantSim.FAGameMode|GetSpacePlane _asfagame_mode))
    (bind _asbp_base_passenger (Utilities|Casting|CastToBP_BasePassenger _array_element))
    (if (<= (Math|Random|RandomFloat) (Variables|Default|GetMakeOrderRate))
      (Default|MakeOrder (Variables|/Game/Characters/BP_BasePassenger.BP_BasePassenger_C|GetOrder%20Component _asbp_base_passenger))
      (bind _asw_character_status (Utilities|Casting|CastToW_CharacterStatus (UserInterface|GetWidget (Variables|/Game/Characters/BP_BasePassenger.BP_BasePassenger_C|GetStatus _asbp_base_passenger))))
      (Default|Init _asw_character_status (Variables|/Game/FoodServing/BP_PassengerOrderComponent.BP_PassengerOrderComponent_C|GetOrder (Variables|/Game/Characters/BP_BasePassenger.BP_BasePassenger_C|GetOrder%20Component _asbp_base_passenger))))))

(event EventBeginPlay
  (bind _foundwidgets (Widget|GetAllWidgetsOfClass "/Game/SpaceShip/PilotCockpit/W_ControlTableDisplay.W_ControlTableDisplay_C" false))
  (Variables|Default|SetControlDisplay (Utilities|Array|Get(acopy) _foundwidgets)))

(event EventOnFlightStart
  (Rendering|Material|SetScalarParameterValue "/Game/Enviroment/Warp/MC_WarpConeParams.MC_WarpConeParams" "Power" 1.0 :!class /Script/Engine.KismetMaterialLibrary)
  (Default|OnFlightStart (Variables|/Game/SpaceShip/PilotCockpit/W_ControlTableDisplay.W_ControlTableDisplay_C|GetW_WeatherRadarWidget (Variables|Default|GetControlDisplay)))
  (CallFunction|MakeOrders)
  (bind _asbp_fagame_mode (Utilities|Casting|CastToBP_FAGameMode (Game|GetGameMode)))
  (Widget|SetIsEnabled (Variables|/Game/UI/W_PauseMenu.W_PauseMenu_C|GetSaveGameButton (Variables|/Game/Blueprints/BP_FAGameMode.BP_FAGameMode_C|GetPauseMenu _asbp_fagame_mode)) false))

(event EventOnFlightEnd
  (Rendering|Material|SetScalarParameterValue "/Game/Enviroment/Warp/MC_WarpConeParams.MC_WarpConeParams" "Power" 0.0 :!class /Script/Engine.KismetMaterialLibrary)
  (Default|OnFlightEnd (Variables|/Game/SpaceShip/PilotCockpit/W_ControlTableDisplay.W_ControlTableDisplay_C|GetW_WeatherRadarWidget (Variables|Default|GetControlDisplay)))
  (bind _asbp_fagame_mode (Utilities|Casting|CastToBP_FAGameMode (Game|GetGameMode)))
  (Widget|SetIsEnabled (Variables|/Game/UI/W_PauseMenu.W_PauseMenu_C|GetSaveGameButton (Variables|/Game/Blueprints/BP_FAGameMode.BP_FAGameMode_C|GetPauseMenu _asbp_fagame_mode)) true))