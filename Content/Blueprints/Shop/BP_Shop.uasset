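; BP_Shop is a shop actor that supplies the items and menu for an in-game shop.
; On BeginPlay it spawns a hidden hyper charger slot actor and a hidden food slot actor, collecting both into a Slots array.
; It then creates the WB_ShopMenu widget, hands it that array and has it build its inventory.
; The ShowShopMenu event adds the prebuilt widget to the viewport and shows the mouse cursor.
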(event Custom|ShowShopMenu
  (UserInterface|Viewport|AddtoViewport (Variables|Default|GetWB_Interface) 0)
  (Variables|/Script/Engine.PlayerController|SetbShowMouseCursor (Game|GetPlayerController 0) true))

(event EventBeginPlay
  (bind _returnvalue (Game|SpawnActorfromClass "/Game/Blueprints/Shop/BP_SlotHyperCharger.BP_SlotHyperCharger_C" (Math|Transform|MakeTransform "0, 0, 0" "0, 0, 0" "1,1,1") "AlwaysSpawn" 0 0))
  (bind _output_get (Variables|Default|SetHyperCharger _returnvalue))
  (Rendering|SetActorHiddenInGame _output_get true)
  (bind _returnvalue_2 (Game|SpawnActorfromClass "/Game/Blueprints/Shop/BP_SlotFood.BP_SlotFood_C" (Math|Transform|MakeTransform "0, 0, 0" "0, 0, 0" "1,1,1") "AlwaysSpawn" 0 0))
  (bind _output_get_2 (Variables|Default|SetFoodSlot1 _returnvalue_2))
  (Rendering|SetActorHiddenInGame _output_get_2 true)
  (Utilities|Array|Add (Variables|Default|GetSlots) (Variables|Default|GetHyperCharger))
  (Utilities|Array|Add (Variables|Default|GetSlots) (Variables|Default|GetFoodSlot1))
  (bind _returnvalue_3 (UserInterface|CreateWidget "/Game/UI/WB_ShopMenu.WB_ShopMenu_C"))
  (bind _output_get_3 (Variables|Default|SetWB_Interface _returnvalue_3))
  (Variables|/Game/UI/WB_ShopMenu.WB_ShopMenu_C|SetSlots _output_get_3 (Variables|Default|GetSlots))
  (Default|CreateInventory _output_get_3))

(fn ConstructionScript)