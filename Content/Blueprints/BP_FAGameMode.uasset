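; BP_FAGameMode is a game mode that hosts a PDA debug display and hooks into the PDA messenger.
; On BeginPlay it creates a hidden W_PDADisplay widget and binds message-received events to a handler that prints the first stored message with its author's name.
; ToggleQuestMenu shows or hides that widget along with the mouse cursor.
; An unconnected weather radar debug widget setup is left unused.
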(event Custom|ShowMessage
  (bind _returnvalue (Class|FAGameMode|GetPDAMessenger))
  (bind _receivedmessages (Variables|/Script/FlightAttendantSim.PDAMessengerComponent|GetReceivedMessages _returnvalue))
  (bind _output (Utilities|Array|Get(acopy) _receivedmessages))
  (Development|PrintString (Utilities|String|ToString(Text) (Utilities|Text|FormatText "{Author}: {Message}" (.characterdisplayname (.author _output)) (.message _output)))))

(event Custom|ToggleQuestMenu
  (bind _returnvalue (Game|GetPlayerController 0))
  (bind _pdadebugwidget (Variables|Default|GetPDADebugWidget))
  (bind _output_get (Variables|Default|SetIsQuestMenuVisible (not (Variables|Default|GetIsQuestMenuVisible))))
  (if _output_get
    (Widget|SetVisibility _pdadebugwidget "Visible")
    (Variables|/Script/Engine.PlayerController|SetbShowMouseCursor _returnvalue true)
    (else
      (Widget|SetVisibility _pdadebugwidget "Hidden")
      (Variables|/Script/Engine.PlayerController|SetbShowMouseCursor _returnvalue false))))

(event EventBeginPlay
  (bind _returnvalue (UserInterface|CreateWidget "/Game/PDA/W_PDADisplay.W_PDADisplay_C"))
  (bind _output_get (Variables|Default|SetPDADebugWidget _returnvalue))
  (Widget|SetVisibility _output_get "Hidden")
  (UserInterface|Viewport|AddtoViewport _output_get 0)
  (EventDispatchers|BindEventtoMessageReceived (Class|FAGameMode|GetPDAMessenger) (delegate Custom|ShowMessage)))

(fn ConstructionScript)