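; BP_PassengerDebug is a placeable marker actor that marks a debug spawn location for passengers.
; On BeginPlay it casts the game mode to BP_FAGameMode and adds itself to that mode's DebugPassengersSpawnLocations collection.
; It has no other active logic, as overlap and tick are disabled and the construction script only calls its parent.
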(event EventBeginPlay
  (bind _asbp_fagame_mode (Utilities|Casting|CastToBP_FAGameMode (Game|GetGameMode)))
  (Utilities|Array|Add (Variables|/Script/FlightAttendantSim.FAGameMode|GetDebugPassengersSpawnLocations _asbp_fagame_mode) self))

(event Collision|EventActorBeginOverlap
  (params (OtherActor :type Actor%20Object%20Reference))
  (|CallParentFunction OtherActor) ; This node is disabled and will not be called.\nDrag off pins to build functionality.
)

(event EventTick
  (params (DeltaSeconds :type Float%20%28single-precision%29))
  (|CallParentFunction DeltaSeconds) ; This node is disabled and will not be called.\nDrag off pins to build functionality.
)

(fn ConstructionScript
  (|CallParentFunction))