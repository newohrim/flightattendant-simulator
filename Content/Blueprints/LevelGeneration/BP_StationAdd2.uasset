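; BP_StationAdd2 is a level-generation actor that spawns a single facility actor when play begins.
; BeginPlay polls on a short delay until the Facility5 class is valid, then spawns it at the Sphere5 component's world location and rotation, ignoring collisions.
; The spawned actor is stored in F1, which the DestroyF event destroys if still valid.
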(event Custom|DestroyF
  (bind _f1 (Variables|Default|Getf1))
  (Utilities|IsValid _f1
    (:Is%20Valid
      (Actor|DestroyActor _f1))))

(event EventBeginPlay
  (bind _sphere5 (Variables|Default|GetSphere5))
  (bind _returnvalue (Transformation|GetSocketTransform _sphere5 "None" "RTS_World"))
  (if (Utilities|IsValidClass (Variables|Default|GetFacility5)) :!label _label
    (bind _returnvalue_2 (Game|SpawnActorfromClass (Variables|Default|GetFacility5) (Math|Transform|MakeTransform (.location _returnvalue) (.rotation _returnvalue) "1,1,1") "AlwaysSpawn" 0 0))
    (Variables|Default|Setf1 _returnvalue_2)
    (else
      (Utilities|FlowControl|Delay 0.2)
      (goto _label))))

(event Collision|EventActorBeginOverlap
  (params (OtherActor :type Actor%20Object%20Reference)))

(event EventTick
  (params (DeltaSeconds :type Float%20%28single-precision%29)))

(fn ConstructionScript)