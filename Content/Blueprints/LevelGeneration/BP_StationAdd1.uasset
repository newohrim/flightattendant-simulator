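; BP_StationAdd1 is a level-generation station piece that spawns facility actors at its sphere markers and adjusts its walls according to a Flag value.
; On BeginPlay it polls with short delays until the facility classes and Flag are set, then spawns Facility3, plus Facility4 for higher Flag values.
; Lower Flag values hide one merged wall and reposition another.
; DestroyF removes both spawned facilities.
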(event Custom|DestroyF
  (bind _f1 (Variables|Default|Getf1))
  (bind _f2 (Variables|Default|Getf2))
  (Utilities|IsValid _f1
    (:Is%20Valid
      (Actor|DestroyActor _f1))
    (:Is%20Not%20Valid
      _))
  (Utilities|IsValid _f2
    (:Is%20Valid
      (Actor|DestroyActor _f2))))

(event EventBeginPlay
  (bind _sphere3 (Variables|Default|GetSphere3))
  (bind _sphere4 (Variables|Default|GetSphere4))
  (bind _returnvalue (Transformation|GetSocketTransform _sphere4 "None" "RTS_World"))
  (bind _returnvalue_2 (Transformation|GetSocketTransform _sphere3 "None" "RTS_World"))
  (Utilities|FlowControl|Sequence
    (:then_0
      (if (Utilities|IsValidClass (Variables|Default|GetFacility3)) :!label _label
        (bind _returnvalue_3 (Game|SpawnActorfromClass (Variables|Default|GetFacility3) (Math|Transform|MakeTransform (.location _returnvalue_2) (.rotation _returnvalue_2) "1,1,1") "AlwaysSpawn" 0 0))
        (Variables|Default|Setf1 _returnvalue_3)
        (else
          (Utilities|FlowControl|Delay 0.2)
          (goto _label))))
    (:then_1
      (if (== (Variables|Default|Getflag) -1) :!label _label_2
        (Utilities|FlowControl|Delay 0.1)
        (goto _label_2)
        (elif (> (Variables|Default|GetFlag) 3)
          (if (Utilities|IsValidClass (Variables|Default|GetFacility4)) :!label _label_3
            (bind _returnvalue_4 (Game|SpawnActorfromClass (Variables|Default|GetFacility4) (Math|Transform|MakeTransform (.location _returnvalue) (.rotation _returnvalue) "1,1,1") "AlwaysSpawn" 0 0))
            (Variables|Default|Setf2 _returnvalue_4)
            (else
              (Utilities|FlowControl|Delay 0.2)
              (goto _label_3))))))
    (:then_2
      (if (== (Variables|Default|GetFlag) -1) :!label _label_4
        (Utilities|FlowControl|Delay 0.2)
        (goto _label_4)
        (elif (not (> (Variables|Default|GetFlag) 4))
          (Rendering|SetVisibility (Variables|Default|GetSM_MERGED_Wall_B_5) false false)
          (Transformation|SetRelativeLocation (Variables|Default|GetSM_MERGED_Wall_B_4) "-1670.000000,-80.000000,-380.000000" false true))))))

(event Collision|EventActorBeginOverlap
  (params (OtherActor :type Actor%20Object%20Reference)))

(event EventTick
  (params (DeltaSeconds :type Float%20%28single-precision%29)))

(fn ConstructionScript)