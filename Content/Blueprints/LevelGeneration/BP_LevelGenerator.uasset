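; Level generator actor that registers itself as the game mode's LocationGenerator and builds a space station from a location's facility list.
; GenerateLocation always spawns the main station, adding the first extension at three or more facilities and the second at five or more, at fixed transforms.
; It passes facility classes to each module, plus the facility count as Flag to the main station and first extension.
; Every facility type currently maps to BP_Shop.
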(event EventGenerateLocation
  (params (LocationInfo :type Location%20Info%20Object%20Reference))
  (Variables|Default|SetFacilities (Variables|/Script/FlightAttendantSim.LocationInfo|GetFacilities LocationInfo))
  (if (< (Utilities|Array|Length (Variables|Default|GetFacilities)) 3)
    _
    (else
      (if (< (Utilities|Array|Length (Variables|Default|GetFacilities)) 5)
        _
        (else
          (bind _returnvalue (Game|SpawnActorfromClass "/Game/Blueprints/LevelGeneration/BP_StationAdd2.BP_StationAdd2_C" (Math|Transform|MakeTransform "3030.000000,-110.000000,20.000000" "0,-90.000000, 0" "0.750000,0.750000,0.750000") "AlwaysSpawn" 0 0))
          (Variables|/Game/Blueprints/LevelGeneration/BP_StationAdd2.BP_StationAdd2_C|SetFacility5 _returnvalue (Utilities|Select :Index (Utilities|Array|Get(acopy) (Variables|Default|GetFacilities) 4) :Shop "/Game/Blueprints/Shop/BP_Shop.BP_Shop_C" :BountyHunter "/Game/Blueprints/Shop/BP_Shop.BP_Shop_C" :CargoShipping "/Game/Blueprints/Shop/BP_Shop.BP_Shop_C" :RepairStation "/Game/Blueprints/Shop/BP_Shop.BP_Shop_C" :RouteGuide "/Game/Blueprints/Shop/BP_Shop.BP_Shop_C" :FACILITY_NR_ITEMS "/Game/Blueprints/Shop/BP_Shop.BP_Shop_C"))))
      (bind _returnvalue_2 (Game|SpawnActorfromClass "/Game/Blueprints/LevelGeneration/BP_StationAdd1.BP_StationAdd1_C" (Math|Transform|MakeTransform "1700.000000,190.000000,20.000000" "0,180.000000, 0" "0.750000,0.750000,0.750000") "AlwaysSpawn" 0 0))
      (Variables|/Game/Blueprints/LevelGeneration/BP_StationAdd1.BP_StationAdd1_C|SetFlag _returnvalue_2 (Utilities|Array|Length (Variables|Default|GetFacilities)))
      (Variables|/Game/Blueprints/LevelGeneration/BP_StationAdd1.BP_StationAdd1_C|SetFacility3 _returnvalue_2 (Utilities|Select :Index (Utilities|Array|Get(acopy) (Variables|Default|GetFacilities) 2) :Shop "/Game/Blueprints/Shop/BP_Shop.BP_Shop_C" :BountyHunter "/Game/Blueprints/Shop/BP_Shop.BP_Shop_C" :CargoShipping "/Game/Blueprints/Shop/BP_Shop.BP_Shop_C" :RepairStation "/Game/Blueprints/Shop/BP_Shop.BP_Shop_C" :RouteGuide "/Game/Blueprints/Shop/BP_Shop.BP_Shop_C" :FACILITY_NR_ITEMS "/Game/Blueprints/Shop/BP_Shop.BP_Shop_C"))
      (if (Utilities|Array|IsValidIndex (Variables|Default|GetFacilities) 3)
        (Variables|/Game/Blueprints/LevelGeneration/BP_StationAdd1.BP_StationAdd1_C|SetFacility4 _returnvalue_2 (Utilities|Select :Index (Utilities|Array|Get(acopy) (Variables|Default|GetFacilities) 3) :Shop "/Game/Blueprints/Shop/BP_Shop.BP_Shop_C" :BountyHunter "/Game/Blueprints/Shop/BP_Shop.BP_Shop_C" :CargoShipping "/Game/Blueprints/Shop/BP_Shop.BP_Shop_C" :RepairStation "/Game/Blueprints/Shop/BP_Shop.BP_Shop_C" :RouteGuide "/Game/Blueprints/Shop/BP_Shop.BP_Shop_C" :FACILITY_NR_ITEMS "/Game/Blueprints/Shop/BP_Shop.BP_Shop_C")))))
  (bind _returnvalue_3 (Game|SpawnActorfromClass "/Game/Blueprints/LevelGeneration/BP_MainStation.BP_MainStation_C" (Math|Transform|MakeTransform "610.000000,280.000000,30.000000" "0,-90.000000, 0" "0.750000,0.750000,0.750000") "AlwaysSpawn" 0 0))
  (Variables|/Game/Blueprints/LevelGeneration/BP_MainStation.BP_MainStation_C|Setflag _returnvalue_3 (Utilities|Array|Length (Variables|Default|GetFacilities)))
  (Variables|/Game/Blueprints/LevelGeneration/BP_MainStation.BP_MainStation_C|SetFacility1 _returnvalue_3 (Utilities|Select :Index (Utilities|Array|Get(acopy) (Variables|Default|GetFacilities)) :Shop "/Game/Blueprints/Shop/BP_Shop.BP_Shop_C" :BountyHunter "/Game/Blueprints/Shop/BP_Shop.BP_Shop_C" :CargoShipping "/Game/Blueprints/Shop/BP_Shop.BP_Shop_C" :RepairStation "/Game/Blueprints/Shop/BP_Shop.BP_Shop_C" :RouteGuide "/Game/Blueprints/Shop/BP_Shop.BP_Shop_C" :FACILITY_NR_ITEMS "/Game/Blueprints/Shop/BP_Shop.BP_Shop_C"))
  (if (Utilities|Array|IsValidIndex (Variables|Default|GetFacilities) 1)
    (Variables|/Game/Blueprints/LevelGeneration/BP_MainStation.BP_MainStation_C|SetFacility2 _returnvalue_3 (Utilities|Select :Index (Utilities|Array|Get(acopy) (Variables|Default|GetFacilities) 1) :Shop "/Game/Blueprints/Shop/BP_Shop.BP_Shop_C" :BountyHunter "/Game/Blueprints/Shop/BP_Shop.BP_Shop_C" :CargoShipping "/Game/Blueprints/Shop/BP_Shop.BP_Shop_C" :RepairStation "/Game/Blueprints/Shop/BP_Shop.BP_Shop_C" :RouteGuide "/Game/Blueprints/Shop/BP_Shop.BP_Shop_C" :FACILITY_NR_ITEMS "/Game/Blueprints/Shop/BP_Shop.BP_Shop_C"))))

(event EventBeginPlay
  ;[1 1 1] Explicit set of actor by LevelGenerator interface
  (bind _asfagame_mode (Utilities|Casting|CastToFAGameMode (Game|GetGameMode)))
  (Variables|/Script/FlightAttendantSim.FAGameMode|SetLocationGenerator _asfagame_mode self))

(fn ConstructionScript)