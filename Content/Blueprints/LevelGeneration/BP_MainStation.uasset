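; BP_MainStation is a level-generation station actor that populates itself with facility actors when play begins.
; It spawns Facility1 at the Sphere1 marker, and Facility2 at Sphere2 if Flag is above 1.
; A Flag of 3 or more also removes the SMWallB10 wall component.
; Delay loops poll until the facility classes are valid and Flag is no longer -1, so those values can be assigned after BeginPlay.
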(event EventBeginPlay
  (bind _sphere1 (Variables|Default|GetSphere1))
  (bind _returnvalue (Transformation|GetSocketTransform _sphere1 "None" "RTS_World"))
  (Utilities|FlowControl|Sequence
    (:then_0
      (if (Utilities|IsValidClass (Variables|Default|GetFacility1)) :!label _label
        (Game|SpawnActorfromClass (Variables|Default|GetFacility1) (Math|Transform|MakeTransform (.location _returnvalue) (.rotation _returnvalue) "1,1,1") "AlwaysSpawn" 0 0)
        (else
          (Utilities|FlowControl|Delay 0.2)
          (goto _label))))
    (:then_1
      (if (== (Variables|Default|Getflag) -1) :!label _label_2
        (Utilities|FlowControl|Delay 0.1)
        (goto _label_2)
        (elif (> (Variables|Default|GetFlag) 1)
          (if (Utilities|IsValidClass (Variables|Default|GetFacility2)) :!label _label_3
            (Game|SpawnActorfromClass (Variables|Default|GetFacility2) (Transformation|GetSocketTransform (Variables|Default|GetSphere2) "None" "RTS_World") "AlwaysSpawn" 0 0)
            (else
              (Utilities|FlowControl|Delay 0.2)
              (goto _label_3))))))
    (:then_2
      (if (== (Variables|Default|GetFlag) -1) :!label _label_4
        (Utilities|FlowControl|Delay 0.2)
        (goto _label_4)
        (elif (not (< (Variables|Default|GetFlag) 3))
          (Components|DestroyComponent (Variables|Default|GetSM_Wall_B10)))))))

(fn ConstructionScript)