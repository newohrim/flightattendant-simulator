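; Base passenger Blueprint that handles document checks and in-flight orders for a passenger.
; Showing documents spawns a BP_PassID filled with the passenger's info and puts the player into inspection; hiding destroys it and reopens dialogue.
; While seated with an order, the passenger can briefly show a status widget on a timer.
; ReceiveObject validates a delivered tray against OrderComponent and completes the order on a match.
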(event Custom|ShowOrder
  (bind _status (Variables|Default|GetStatus))
  (bind _returnvalue (UserInterface|GetWidget _status))
  (if (and (> (Utilities|Array|Length (Variables|/Game/FoodServing/BP_PassengerOrderComponent.BP_PassengerOrderComponent_C|GetOrder (Variables|Default|GetOrder%20Component))) 0) (Variables|Default|GetIsSitting))
    (if (not (Widget|IsVisible _returnvalue))
      (Widget|SetVisibility _returnvalue "Visible")
      (Utilities|Time|SetTimerbyEvent (delegate Custom|HideOrder) 5.0))))

(event Custom|HideOrder
  (Widget|SetVisibility (UserInterface|GetWidget (Variables|Default|GetStatus)) "Hidden"))

(event EventBeginPlay
  (|CallParentFunction)
  (Widget|SetVisibility (UserInterface|GetWidget (Variables|Default|GetStatus)) "Hidden"))

(event Collision|EventActorBeginOverlap
  (params (OtherActor :type Actor%20Object%20Reference))
  (|CallParentFunction OtherActor) ; This node is disabled and will not be called.\nDrag off pins to build functionality.
)

(event EventTick
  (params (DeltaSeconds :type Float%20%28single-precision%29))
  (|CallParentFunction DeltaSeconds) ; This node is disabled and will not be called.\nDrag off pins to build functionality.
)

(event EventShowDocuments
  (|CallParentFunction)
  (bind _returnvalue (Game|SpawnActorfromClass "/Game/DocumentsCheck/BP_PassID.BP_PassID_C" (Transformation|GetWorldTransform (Variables|Default|GetPassIdSpawnPoint)) "AlwaysSpawn" 0 0))
  (bind _output_get (Variables|Default|SetSpawnedPassId _returnvalue))
  (Variables|/Game/DocumentsCheck/BP_PassID.BP_PassID_C|SetOwningPassenger _output_get self)
  (bind _asw_pass_idwidget (Utilities|Casting|CastToW_PassIDWidget (UserInterface|GetWidget (Variables|/Game/DocumentsCheck/BP_PassID.BP_PassID_C|GetPassWidget _output_get))))
  (Variables|/Game/DocumentsCheck/UI/W_PassIDWidget.W_PassIDWidget_C|SetDocInfo _asw_pass_idwidget (Variables|Default|GetDocumentsInfo))
  (Variables|/Game/DocumentsCheck/UI/W_PassIDWidget.W_PassIDWidget_C|SetPassIdObject _asw_pass_idwidget _output_get)
  (bind _asfirst_person_character (Utilities|Casting|CastToFirstPersonCharacter (Game|GetPlayerCharacter 0)))
  (Default|OnDialogueOut (Variables|/Game/FirstPersonBP/Blueprints/FirstPersonCharacter.FirstPersonCharacter_C|GetCameraTracerComponent _asfirst_person_character))
  (Default|InspectObject _asfirst_person_character _output_get))

(event EventUnShowDocuments
  (params (IsApproved :type Boolean))
  (bind _spawnedpassid (Variables|Default|GetSpawnedPassId))
  (|CallParentFunction IsApproved)
  (Utilities|IsValid _spawnedpassid
    (:Is%20Valid
      (Actor|DestroyActor _spawnedpassid)
      (bind _asfirst_person_character (Utilities|Casting|CastToFirstPersonCharacter (Game|GetPlayerCharacter 0)))
      (Default|UnInspectObject _asfirst_person_character)
      (Default|OpenDialogueWindow (Variables|/Game/FirstPersonBP/Blueprints/FirstPersonCharacter.FirstPersonCharacter_C|GetCameraTracerComponent _asfirst_person_character) (Variables|Default|GetDialogueComponent))
      (Default|OnDialoguein (Variables|/Game/FirstPersonBP/Blueprints/FirstPersonCharacter.FirstPersonCharacter_C|GetCameraTracerComponent _asfirst_person_character)))))

(fn ConstructionScript
  (|CallParentFunction))

(fn ReceiveObject
  (params (ReceivedObject :type Object%20Object%20Reference))
  (Utilities|IsValid ReceivedObject
    (:Is%20Valid
      (bind _asbp_tray (Utilities|Casting|CastToBP_Tray ReceivedObject))
      (if (Variables|Default|GetIsSitting)
        (if (Default|ValidateOrder (Variables|Default|GetOrder%20Component) (Default|GetTrayContent _asbp_tray))
          (Default|CompleteOrder (Variables|Default|GetOrder%20Component))
          (return true)
          (else
            (return false)))))
    (:Is%20Not%20Valid
      (return false))))