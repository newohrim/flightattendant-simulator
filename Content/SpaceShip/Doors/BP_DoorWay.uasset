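; BP_DoorWay is a spaceship sliding double door that opens for characters and closes when none remain.
; OpenTrigger overlaps maintain a list of characters inside, so the doors close only once it is empty.
; Opening and closing share one MoveComponentTo per door, with a Direction flag selecting either the offset outer spot markers or the positions cached at BeginPlay.
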(event OnComponentBeginOverlap(OpenTrigger)
  (params (OverlappedComponent :type Primitive%20Component%20Object%20Reference) (OtherActor :type Actor%20Object%20Reference) (OtherComp :type Primitive%20Component%20Object%20Reference) (OtherBodyIndex :type Integer) (bFromSweep :type Boolean) (SweepResult :type Hit%20Result%20Structure%20%28by%20ref%29))
  (bind _ascharacter (Utilities|Casting|CastToCharacter OtherActor))
  (Utilities|Array|AddUnique (Variables|Default|GetContent) _ascharacter)
  (CallFunction|OpenDoors))

(event OnComponentEndOverlap(OpenTrigger)
  (params (OverlappedComponent :type Primitive%20Component%20Object%20Reference) (OtherActor :type Actor%20Object%20Reference) (OtherComp :type Primitive%20Component%20Object%20Reference) (OtherBodyIndex :type Integer))
  (bind _ascharacter (Utilities|Casting|CastToCharacter OtherActor))
  (Utilities|Array|RemoveItem (Variables|Default|GetContent) _ascharacter)
  (CallFunction|CloseDoors))

(event Custom|OpenDoors
  (bind _rightdoor (Variables|Default|GetRightDoor))
  (bind _rightmostspot (Variables|Default|GetRightMostSpot))
  (bind _leftdoor (Variables|Default|GetLeftDoor))
  (bind _leftmostspot (Variables|Default|GetLeftMostSpot))
  (bind _relativelocation (Variables|/Script/Engine.SceneComponent|GetRelativeLocation _rightmostspot))
  (bind _relativelocation_2 (Variables|/Script/Engine.SceneComponent|GetRelativeLocation _leftmostspot))
  (if (not (Variables|Default|GetIsOpened))
    (Variables|Default|SetIsOpened true)
    (Variables|Default|SetDirection true)
    (Utilities|FlowControl|Sequence
      (:then_0
        (Components|MoveComponentTo _leftdoor (select (Variables|Default|GetDirection) (Math|Vector|MakeVector (+ (.x _relativelocation_2) -5.0) (.y _relativelocation_2) (.z _relativelocation_2)) (Variables|Default|GetLeftDoorInitPos)) (Variables|/Script/Engine.SceneComponent|GetRelativeRotation _leftdoor) false false 0.2 false))
      (:then_1
        (Components|MoveComponentTo _rightdoor (select (Variables|Default|GetDirection) (Math|Vector|MakeVector (+ (.x _relativelocation) 5.0) (.y _relativelocation) (.z _relativelocation)) (Variables|Default|GetRightDoorInitPos)) (Variables|/Script/Engine.SceneComponent|GetRelativeRotation _rightdoor) false false 0.2 false)))))

(event Custom|CloseDoors
  (bind _rightdoor (Variables|Default|GetRightDoor))
  (bind _rightmostspot (Variables|Default|GetRightMostSpot))
  (bind _leftdoor (Variables|Default|GetLeftDoor))
  (bind _leftmostspot (Variables|Default|GetLeftMostSpot))
  (bind _relativelocation (Variables|/Script/Engine.SceneComponent|GetRelativeLocation _rightmostspot))
  (bind _relativelocation_2 (Variables|/Script/Engine.SceneComponent|GetRelativeLocation _leftmostspot))
  (if (and (Variables|Default|GetIsOpened) (== (Utilities|Array|Length (Variables|Default|GetContent)) 0))
    (Variables|Default|SetIsOpened false)
    (Variables|Default|SetDirection false)
    (Utilities|FlowControl|Sequence
      (:then_0
        (Components|MoveComponentTo _leftdoor (select (Variables|Default|GetDirection) (Math|Vector|MakeVector (+ (.x _relativelocation_2) -5.0) (.y _relativelocation_2) (.z _relativelocation_2)) (Variables|Default|GetLeftDoorInitPos)) (Variables|/Script/Engine.SceneComponent|GetRelativeRotation _leftdoor) false false 0.2 false))
      (:then_1
        (Components|MoveComponentTo _rightdoor (select (Variables|Default|GetDirection) (Math|Vector|MakeVector (+ (.x _relativelocation) 5.0) (.y _relativelocation) (.z _relativelocation)) (Variables|Default|GetRightDoorInitPos)) (Variables|/Script/Engine.SceneComponent|GetRelativeRotation _rightdoor) false false 0.2 false)))))

(event EventBeginPlay
  (Variables|Default|SetLeftDoorInitPos (Variables|/Script/Engine.SceneComponent|GetRelativeLocation (Variables|Default|GetLeftDoor)))
  (Variables|Default|SetRightDoorInitPos (Variables|/Script/Engine.SceneComponent|GetRelativeLocation (Variables|Default|GetRightDoor))))

(fn ConstructionScript)