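; Game mode that runs a flight-attendant game through three phases: document check, briefing and serving, ending in a final score screen.
; Phase events switch possessed pawn, camera and UI, while document handlers forward to a passenger traffic manager and briefing hits score through the game state.
; Timed phases bind penalty dispatchers on timeout, which Tick fires every frame until completion unbinds them.
; BeginPlay also creates a test quest and toggleable debug quest menu.
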(event Custom|Start%20Game
  (bind _mainwidget (Variables|Default|GetMainWidget))
  (Variables|Default|SetCurrentPhase 1)
  (bind _returnvalue (Utilities|Time|SetTimerbyEvent (delegate Custom|DocumentsCheckPhaseTimeLimitExceded) (Variables|Default|GetDocumentsCheckTimePhase)))
  (Variables|/Game/DocumentsCheckOld/UI/W_DocumentsCheckUI.W_DocumentsCheckUI_C|SetCurrentPhaseTimer _mainwidget _returnvalue)
  (Variables|/Game/DocumentsCheckOld/UI/W_DocumentsCheckUI.W_DocumentsCheckUI_C|SetPhaseTime _mainwidget (Variables|Default|GetDocumentsCheckTimePhase))
  (Default|StartPhase1 (Variables|Default|GetMainWidget))
  (CallFunction|LetNextPassenger))

(event Custom|DocumentsCheckPhaseTimeLimitExceded
  (if (== (Variables|Default|GetCurrentPhase) 1)
    (EventDispatchers|BindEventtoDocumentsCheckPhasePenaltyRun (EventDispatchers|CreateEvent :!event AddPenalty))))

(event Custom|ResetLevelExecute
  (Game|OpenLevel(byObjectReference) "/Game/FirstPersonBP/Maps/FirstPersonExampleMap.FirstPersonExampleMap"))

(event Custom|ExitToMainMenu
  (Game|OpenLevel(byObjectReference) "/Game/FirstPersonBP/Maps/MainMenu.MainMenu"))

(event Custom|ToggleQuestMenu
  (bind _returnvalue (Game|GetPlayerController 0))
  (bind _questmenudebugwidget (Variables|Default|GetQuestMenuDebugWidget))
  (bind _output_get (Variables|Default|SetIsQuestMenuVisible (not (Variables|Default|GetIsQuestMenuVisible))))
  (if _output_get
    (Widget|SetVisibility _questmenudebugwidget "Visible")
    (Variables|/Script/Engine.PlayerController|SetbShowMouseCursor _returnvalue true)
    (else
      (Widget|SetVisibility _questmenudebugwidget "Hidden")
      (Variables|/Script/Engine.PlayerController|SetbShowMouseCursor _returnvalue false))))

(event Custom|BriefingPhaseStart
  (Default|StartPhase2 (Variables|Default|GetMainWidget))
  (bind _returnvalue (Actor|GetActorOfClass "/Game/BriefingDemo/Blueprints/BP_Pawn.BP_Pawn_C"))
  (Pawn|Possess (Game|GetPlayerController 0) _returnvalue)
  (Default|StartPhase (Variables|/Game/BriefingDemo/Blueprints/BP_Pawn.BP_Pawn_C|GetBriefingComponent _returnvalue))
  (bind _outactors (Actor|GetAllActorsOfClass "/Game/BriefingDemo/Blueprints/BP_Spawner.BP_Spawner_C"))
  (for _array_element _outactors
    (Actor|Tick|SetActorTickEnabled _array_element true))
  (bind _returnvalue_2 (Actor|GetActorOfClass "/Game/BriefingDemo/Blueprints/BP_Camera.BP_Camera_C"))
  (Game|Player|SetViewTargetwithBlend (Game|GetPlayerController 0) _returnvalue_2 0.0 "VTBlend_Linear" 0.0 false)
  ;[1 1 1] Briefing UI
  (bind _returnvalue_3 (UserInterface|CreateWidget "/Game/BriefingDemo/Blueprints/UI/W_BriefingUI.W_BriefingUI_C"))
  (UserInterface|Viewport|AddtoViewport _returnvalue_3 0))

(event Custom|DocumentsCheckPhaseCompleted
  (Variables|Default|SetCurrentPhase 2)
  (EventDispatchers|UnbindallEventsfromDocumentsCheckPhasePenaltyRun)
  (Utilities|FlowControl|Delay 5.0)
  (CallFunction|BriefingPhaseStart))

(event Custom|ServingPhaseStart
  (bind _mainwidget (Variables|Default|GetMainWidget))
  (Variables|Default|SetCurrentPhase 3)
  (bind _returnvalue (Actor|GetActorOfClass "/Game/FirstPersonBP/Blueprints/FirstPersonCharacter.FirstPersonCharacter_C"))
  (Variables|/Game/FirstPersonBP/Blueprints/FirstPersonCharacter.FirstPersonCharacter_C|SetCanBeQuested _returnvalue true)
  (bind _returnvalue_2 (Utilities|Time|SetTimerbyEvent (delegate Custom|ServingPhaseTimeOut) (Variables|Default|GetServingPhaseTime)))
  (Variables|/Game/DocumentsCheckOld/UI/W_DocumentsCheckUI.W_DocumentsCheckUI_C|SetCurrentPhaseTimer _mainwidget _returnvalue_2)
  (Variables|/Game/DocumentsCheckOld/UI/W_DocumentsCheckUI.W_DocumentsCheckUI_C|SetPhaseTime _mainwidget (Variables|Default|GetServingPhaseTime))
  (Default|StartPhase3 (Variables|Default|GetMainWidget)))

(event Custom|ServingPhaseTimeOut
  (if (== (Variables|Default|GetCurrentPhase) 3)
    (EventDispatchers|BindEventtoServingPhasePenaltyRun (EventDispatchers|CreateEvent :!event AddPenaltyServing))))

(event Custom|BriefingGoodHit
  (Default|BriefingGivePoints (Variables|Default|GetGlobalGameState)))

(event Custom|ServingPhaseCompeted
  (EventDispatchers|UnbindallEventsfromServingPhasePenaltyRun)
  (bind _asbp_controller (Utilities|Casting|CastToBP_Controller (Game|GetPlayerController 0)))
  (Default|IgnorePlayerInput _asbp_controller)
  (bind _returnvalue (UserInterface|CreateWidget "/Game/UI/W_FinalScore.W_FinalScore_C" _asbp_controller))
  (UserInterface|Viewport|AddtoViewport _returnvalue 1)
  (Variables|/Script/Engine.PlayerController|SetbShowMouseCursor (Game|GetPlayerController 0) true))

(event Custom|BriefingBadHit
  (Default|BriefingGivePenalty (Variables|Default|GetGlobalGameState)))

(event Custom|BriefingPhaseCompleted
  (Utilities|FlowControl|Delay 3.0)
  (Development|PrintString "Phase completed")
  (bind _returnvalue (Actor|GetActorOfClass "/Game/FirstPersonBP/Blueprints/FirstPersonCharacter.FirstPersonCharacter_C"))
  (Pawn|Possess (Game|GetPlayerController 0) _returnvalue)
  (bind _foundwidgets (Widget|GetAllWidgetsOfClass "/Game/BriefingDemo/Blueprints/UI/W_BriefingUI.W_BriefingUI_C" true))
  (Widget|RemovefromParent (Utilities|Array|Get(acopy) _foundwidgets))
  (CallFunction|ServingPhaseStart))

(event EventBeginPlay
  (bind _returnvalue (Game|GetPlayerController 0))
  ;[1 1 1] Quest Test Debug
  (bind _returnvalue_2 (Game|ConstructObjectfromClass (Variables|Default|GetTestQuest) self))
  (bind _asq_test_quest (Utilities|Casting|CastToQ_TestQuest _returnvalue_2))
  (bind _output_get (Variables|Default|SetTestQuest2 _asq_test_quest))
  (bind _returnvalue_3 (Actor|GetActorOfClass "/Game/DocumentsCheckOld/BP_PlaneDoor.BP_PlaneDoor_C"))
  (Variables|/Game/Quests/TestQuests/Q_TestQuest.Q_TestQuest_C|SetPlaneDoor _output_get _returnvalue_3)
  (Class|Quest|Init _output_get)
  (Class|Quest|TakeQuest _output_get)
  ;[1 1 1] QuestMenu Debug
  (bind _returnvalue_4 (UserInterface|CreateWidget "/Game/PDA/W_QuestMenu.W_QuestMenu_C"))
  (UserInterface|Viewport|AddtoViewport _returnvalue_4 0)
  (bind _output_get_2 (Variables|Default|SetQuestMenuDebugWidget _returnvalue_4))
  (Widget|SetVisibility _output_get_2 "Hidden")
  (bind _asbp_fabase_game_state (Utilities|Casting|CastToBP_FABaseGameState (Game|GetGameState)))
  (Variables|Default|SetGlobalGameState _asbp_fabase_game_state)
  (bind _returnvalue_5 (Actor|GetActorOfClass "/Game/FirstPersonBP/Blueprints/FirstPersonCharacter.FirstPersonCharacter_C"))
  (Pawn|Possess _returnvalue _returnvalue_5)
  (Game|Player|SetViewTargetwithBlend _returnvalue _returnvalue_5 0.0 "VTBlend_EaseIn" 1.0 false))

(event EventTick
  (params (DeltaSeconds :type Float%20%28single-precision%29))
  (Default|CallDocumentsCheckPhasePenaltyRun)
  (Default|CallServingPhasePenaltyRun))

(fn ConstructionScript)

(fn LetNextPassenger
  (bind _passengerstrafficmanager (Variables|Default|GetPassengersTrafficManager)
    (:then
      (Default|NextPassenger _passengerstrafficmanager))
    (:else
      (Development|PrintString "PassengersTraffic was not set"))))

(fn DocumentApprovedHandler
  (bind _passengerstrafficmanager (Variables|Default|GetPassengersTrafficManager)
    (:then
      (Default|OnDocsApproval _passengerstrafficmanager))
    (:else
      (Development|PrintString "PassengersTraffic was not set"))))

(fn DocumentDisapprovedHandler
  (bind _passengerstrafficmanager (Variables|Default|GetPassengersTrafficManager)
    (:then
      (Default|OnDocsDisapproval _passengerstrafficmanager))
    (:else
      (Development|PrintString "PassengersTraffic was not set"))))

(fn GetPlayerScore
  (return (Math|Float|Clamp(Float) (- (* 100 (/ (Math|Conversions|ToFloat(Integer) (Variables|Default|GetPlayersScore)) (Math|Conversions|ToFloat(Integer) (Variables|Default|GetPlayersMaxScore)))) (Variables|Default|GetCurrentPenalty)) 0.0 1e+02)))

(fn AddPenalty
  (Variables|Default|SetCurrentPenalty (+ (Variables|Default|GetCurrentPenalty) (* (Variables|Default|GetScorePenaltyPerSec) (Utilities|Time|GetWorldDeltaSeconds)))))

(fn AddPenaltyServing
  (Default|ServingGivePenalty (Variables|Default|GetGlobalGameState)))