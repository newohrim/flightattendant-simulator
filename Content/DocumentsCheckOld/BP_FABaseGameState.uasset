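; BP_FABaseGameState is a game state that tracks world time and scores for the briefing and passenger-serving phases.
; Tick advances the world clock at ten times real time, while briefing events update a percentage of good versus bad figures.
; Serving penalties drain a clamped score scaled by frame time, reported as a percentage of three points per passenger.
; Once every passenger is served, it notifies BP_FABaseGameMode that serving is complete.
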(event Custom|ServingGivePenalty
  (Variables|Default|SetServingScore (Math|Float|Clamp(Float) (- (Variables|Default|GetServingScore) (* (Variables|Default|GetPenaltyAmount) (Utilities|Time|GetWorldDeltaSeconds))) 0.0 (Math|Conversions|ToFloat(Integer) (* (Variables|Default|GetPassengersCount) 3)))))

(event Custom|BriefingGivePenalty
  (bind _output_get (Variables|Default|SetBadFigures (+ (Variables|Default|GetBadFigures) 1)))
  (Development|PrintString "Bad" true true "(R=1.000000,G=0.058804,B=0.138485,A=1.000000)")
  (Variables|Default|SetBriefingScore (* 100 (/ (Math|Conversions|ToFloat(Integer) (stale Custom|BriefingGivePoints _output_get)) (Math|Conversions|ToFloat(Integer) (+ (stale Custom|BriefingGivePoints _output_get) _output_get))))))

(event Custom|BriefingGivePoints
  (bind _output_get (Variables|Default|SetGoodFigures (+ (Variables|Default|GetGoodFigures) 1)))
  (Development|PrintString "Good" true true "(R=0.200115,G=1.000000,B=0.000000,A=1.000000)")
  (Variables|Default|SetBriefingScore (* 100 (/ (Math|Conversions|ToFloat(Integer) _output_get) (Math|Conversions|ToFloat(Integer) (+ _output_get (stale Custom|BriefingGivePenalty _output_get)))))))

(event EventBeginPlay)

(event EventTick
  (params (DeltaSeconds :type Float%20%28single-precision%29))
  (Variables|Default|SetWorldDateTime (+ (Variables|Default|GetWorldDateTime) (Math|Timespan|MakeTimespan 0 0 0 0 (Math|Float|Truncate (* 10000 DeltaSeconds))))))

(fn ConstructionScript)

(fn GetServingScore
  (return (* 100 (/ (Variables|Default|GetServingScore) (Math|Conversions|ToFloat(Integer) (* (Variables|Default|GetPassengersCount) 3))))))

(fn AddServedPassenger
  (bind _output_get (Variables|Default|SetServedPassengers (+ (Variables|Default|GetServedPassengers) 1)))
  (if (== _output_get (Variables|Default|GetPassengersCount))
    (bind _asbp_fabase_game_mode (Utilities|Casting|CastToBP_FABaseGameMode (Game|GetGameMode)))
    (Default|ServingPhaseCompeted _asbp_fabase_game_mode)))