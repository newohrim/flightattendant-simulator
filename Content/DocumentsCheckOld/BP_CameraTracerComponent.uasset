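; Player interaction component that line-traces from the owner's camera to drive pickup and use of world objects.
; TryPick grabs pickables or spawns from dispensers; TryInteract dispatches by cast to carts, interactables, characters, toilets, shops, and wire and tube puzzles.
; Characters receive held items or open a dialogue widget that locks player input.
; It also shows passenger order tooltips each tick, requests orders, controls kettle leaning and zooms the control-table map.
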(event Custom|DropPickedObject
  (bind _pickedobject (Variables|Default|GetPickedObject))
  (Utilities|IsValid _pickedobject
    (:Is%20Valid
      (Default|Drop _pickedobject)
      (Variables|/Script/Engine.CameraComponent|SetbUsePawnControlRotation (Variables|Default|GetPlayer%20Camera) true)
      (bind _asfirst_person_character (Utilities|Casting|CastToFirstPersonCharacter (Components|GetOwner)))
      (Default|OnItemDropped _asfirst_person_character))))

(event Custom|TryPick
  (bind _player_camera (Variables|Default|GetPlayer%20Camera))
  (bind _returnvalue (Transformation|GetWorldLocation _player_camera))
  (Utilities|IsValid (Variables|Default|GetPickedObject)
    (:Is%20Valid
      (if (Variables|/Game/FoodServing/BP_BasePickableObject.BP_BasePickableObject_C|GetIsPicked? (Variables|Default|GetPickedObject))
        (CallFunction|DropPickedObject)
        (else
          (bind (_outhit _returnvalue_2) (Collision|LineTraceByChannel _returnvalue (+ _returnvalue (* (Math|Vector|GetForwardVector (Variables|Default|GetPlayer%20Camera)) (Variables|Default|GetTraceDistance))) "TraceTypeQuery2" false 0 "None" :!label _label))
          (if _returnvalue_2
            (Development|PrintString (Utilities|GetDisplayName (.HitActor (Collision|BreakHitResult _outhit))))
            (bind _asbp_base_pickable_object (Utilities|Casting|CastToBP_BasePickableObject (.HitActor (Collision|BreakHitResult _outhit)))
              (:then
                (Default|PickUp _asbp_base_pickable_object (Variables|Default|GetPlayer%20Camera) self)
                (Variables|Default|SetPickedObject _asbp_base_pickable_object)
                (bind _asfirst_person_character (Utilities|Casting|CastToFirstPersonCharacter (Components|GetOwner)))
                (Default|OnItemPicked _asfirst_person_character))
              (:CastFailed
                (bind _asbp_dispenser (Utilities|Casting|CastToBP_Dispenser (.HitActor (Collision|BreakHitResult _outhit))))
                (Default|CreateInstance _asbp_dispenser self)))))))
    (:Is%20Not%20Valid
      (goto _label))))

(event Custom|TryInteract
  (bind _pickedobject (Variables|Default|GetPickedObject))
  (bind _player_camera (Variables|Default|GetPlayer%20Camera))
  (bind _returnvalue (Transformation|GetWorldLocation _player_camera))
  (Utilities|IsValid (Variables|Default|GetEscortedCart)
    (:Is%20Valid
      (if (Variables|/Game/FoodServing/BP_Cart.BP_Cart_C|GetIsEscorting? (Variables|Default|GetEscortedCart))
        (Default|EscortEnd (Variables|Default|GetEscortedCart))
        (else
          (if (Variables|Default|GetIsTalking) :!label _label
            (CallFunction|OnDialogueOut)
            (else
              (bind (_outhit _returnvalue_2) (Collision|LineTraceByChannel _returnvalue (+ _returnvalue (* (Math|Vector|GetForwardVector (Variables|Default|GetPlayer%20Camera)) (Variables|Default|GetTraceDistance))) "TraceTypeQuery1" false 0 "None"))
              (if _returnvalue_2
                (Development|PrintString (Utilities|GetDisplayName (.HitActor (Collision|BreakHitResult _outhit))))
                (bind _asbp_cart (Utilities|Casting|CastToBP_Cart (.HitActor (Collision|BreakHitResult _outhit)))
                  (:then
                    (bind _asfirst_person_character (Utilities|Casting|CastToFirstPersonCharacter (Components|GetOwner)))
                    (Default|EscortStart _asbp_cart _asfirst_person_character)
                    (Variables|Default|SetEscortedCart _asbp_cart))
                  (:CastFailed
                    (bind _asbp_base_interactable_object (Utilities|Casting|CastToBP_BaseInteractableObject (.HitActor (Collision|BreakHitResult _outhit)))
                      (:then
                        (Default|Interact _asbp_base_interactable_object))
                      (:CastFailed
                        (bind _asfabase_character (Utilities|Casting|CastToFABaseCharacter (.HitActor (Collision|BreakHitResult _outhit)))
                          (:then
                            (Utilities|IsValid _pickedobject
                              (:Is%20Valid
                                (if (Variables|/Game/FoodServing/BP_BasePickableObject.BP_BasePickableObject_C|GetIsPicked? _pickedobject)
                                  (CallFunction|GiveObjectHandle (Variables|Default|GetPickedObject) _asfabase_character)
                                  (else
                                    (if (not (Variables|Default|GetIsTalking)) :!label _label_2
                                      (CallFunction|OnDialoguein)
                                      (Utilities|IsValid (Variables|/Script/FlightAttendantSim.DialogueComponent|GetDialogueContext (Variables|/Script/FlightAttendantSim.FABaseCharacter|GetDialogueComponent _asfabase_character))
                                        (:Is%20Valid
                                          _)
                                        (:Is%20Not%20Valid
                                          (Class|FABaseCharacter|Talkto _asfabase_character (Components|GetOwner))))
                                      (CallFunction|OpenDialogueWindow (Variables|/Script/FlightAttendantSim.FABaseCharacter|GetDialogueComponent _asfabase_character))
                                      (Class|ActionExecutorComponent|PauseCurrentAction (Variables|/Script/FlightAttendantSim.FABaseCharacter|GetActionExecutorComponent _asfabase_character))
                                      (EventDispatchers|BindEventtoOnDialogueOutDispatcher (EventDispatchers|CreateEvent (Variables|/Script/FlightAttendantSim.FABaseCharacter|GetActionExecutorComponent _asfabase_character) :!event ResumeCurrentAction))))))
                              (:Is%20Not%20Valid
                                (goto _label_2))))
                          (:CastFailed
                            (bind _asbp_toilet (Utilities|Casting|CastToBP_Toilet (.HitActor (Collision|BreakHitResult _outhit)))
                              (:then
                                (Default|ClearContent _asbp_toilet))
                              (:CastFailed
                                (bind _asbp_shop (Utilities|Casting|CastToBP_Shop (.HitActor (Collision|BreakHitResult _outhit)))
                                  (:then
                                    (Default|ShowShopMenu _asbp_shop)
                                    (bind _asfirst_person_character_2 (Utilities|Casting|CastToFirstPersonCharacter (Game|GetPlayerCharacter 0)))
                                    (Variables|/Game/FirstPersonBP/Blueprints/FirstPersonCharacter.FirstPersonCharacter_C|SetInspectionMode _asfirst_person_character_2 true))
                                  (:CastFailed
                                    (bind _asfirst_person_character_3 (Utilities|Casting|CastToFirstPersonCharacter (Game|GetPlayerCharacter 0)))
                                    (if (Variables|/Game/FirstPersonBP/Blueprints/FirstPersonCharacter.FirstPersonCharacter_C|GetWiresCatched _asfirst_person_character_3)
                                      (bind _asbp_wire_system (Utilities|Casting|CastToBP_WireSystem (.HitActor (Collision|BreakHitResult _outhit)) :!label _label_3)
                                        (:then
                                          (bind _asstatic_mesh_component (Utilities|Casting|CastToStaticMeshComponent (.HitComponent (Collision|BreakHitResult _outhit))))
                                          (bind _output_get (Variables|Default|SetwireButton _asstatic_mesh_component))
                                          (if (== _asstatic_mesh_component (Variables|/Game/Blueprints/MiniGames/BP_WireSystem.BP_WireSystem_C|GetOuterButton _asbp_wire_system))
                                            (Default|OpenBox _asbp_wire_system)
                                            (elif (== _asstatic_mesh_component (Variables|/Game/Blueprints/MiniGames/BP_WireSystem.BP_WireSystem_C|GetInnerButton _asbp_wire_system))
                                              (Default|CloseBox _asbp_wire_system)
                                              (elif (Math|Boolean|ORBoolean (== (Variables|/Game/Blueprints/MiniGames/BP_WireSystem.BP_WireSystem_C|Getgreen1 _asbp_wire_system) _output_get) (== _output_get (Variables|/Game/Blueprints/MiniGames/BP_WireSystem.BP_WireSystem_C|Getgreen2 _asbp_wire_system)) (== _output_get (Variables|/Game/Blueprints/MiniGames/BP_WireSystem.BP_WireSystem_C|Getred1 _asbp_wire_system)) (== (Variables|/Game/Blueprints/MiniGames/BP_WireSystem.BP_WireSystem_C|Getred2 _asbp_wire_system) _output_get) (== (Variables|/Game/Blueprints/MiniGames/BP_WireSystem.BP_WireSystem_C|Getblue1 _asbp_wire_system) _output_get) (== (Variables|/Game/Blueprints/MiniGames/BP_WireSystem.BP_WireSystem_C|Getblue2 _asbp_wire_system) _output_get))
                                                (bind _asfirst_person_character_4 (Utilities|Casting|CastToFirstPersonCharacter (Game|GetPlayerCharacter 0)))
                                                (if (Variables|/Game/FirstPersonBP/Blueprints/FirstPersonCharacter.FirstPersonCharacter_C|GetWiresCatched _asfirst_person_character_4)
                                                  (if (== (Variables|Default|Getsphere) (Variables|/Game/Blueprints/MiniGames/BP_Wires.BP_Wires_C|GetSphereA (Variables|Default|GetAs%20BP%20Wires)))
                                                    (Class|PhysicsConstraintComponent|SetConstrainedComponents (Variables|/Game/Blueprints/MiniGames/BP_Wires.BP_Wires_C|GetPhysicsConstraintA (Variables|Default|GetAs%20BP%20Wires)) (Variables|/Game/Blueprints/MiniGames/BP_Wires.BP_Wires_C|GetSphereA (Variables|Default|GetAs%20BP%20Wires)) "None" (Variables|Default|GetwireButton) "None")
                                                    (Variables|/Game/FirstPersonBP/Blueprints/FirstPersonCharacter.FirstPersonCharacter_C|SetWiresCatched _asfirst_person_character_4 false)
                                                    (elif (== (Variables|Default|Getsphere) (Variables|/Game/Blueprints/MiniGames/BP_Wires.BP_Wires_C|GetSphereB (Variables|Default|GetAs%20BP%20Wires)))
                                                      (Class|PhysicsConstraintComponent|SetConstrainedComponents (Variables|/Game/Blueprints/MiniGames/BP_Wires.BP_Wires_C|GetPhysicsConstraintB (Variables|Default|GetAs%20BP%20Wires)) (Variables|/Game/Blueprints/MiniGames/BP_Wires.BP_Wires_C|GetSphereB (Variables|Default|GetAs%20BP%20Wires)) "None" (Variables|Default|GetwireButton) "None")
                                                      (Variables|/Game/FirstPersonBP/Blueprints/FirstPersonCharacter.FirstPersonCharacter_C|SetWiresCatched _asfirst_person_character_4 false))))))))
                                        (:CastFailed
                                          (bind _asbp_tube_system (Utilities|Casting|CastToBP_TubeSystem (.HitActor (Collision|BreakHitResult _outhit)))
                                            (:then
                                              (bind _asstatic_mesh_component_2 (Utilities|Casting|CastToStaticMeshComponent (.HitComponent (Collision|BreakHitResult _outhit))))
                                              (bind _output_get_2 (Variables|Default|SettubeButton _asstatic_mesh_component_2))
                                              (if (== _output_get_2 0)
                                                (Default|OpenBoxRight _asbp_tube_system)
                                                (elif (== _output_get_2 0)
                                                  (Default|OpenBoxLeft _asbp_tube_system)
                                                  (elif (== (Variables|/Game/Blueprints/MiniGames/BP_TubeSystem.BP_TubeSystem_C|GetInnerButton _asbp_tube_system) _output_get_2)
                                                    (Utilities|FlowControl|Sequence
                                                      (:then_0
                                                        (Default|CloseBoxRight _asbp_tube_system))
                                                      (:then_1
                                                        (Default|CloseBoxLeft _asbp_tube_system)))))))
                                            (:CastFailed
                                              (bind _asbp_tube (Utilities|Casting|CastToBP_Tube (.HitActor (Collision|BreakHitResult _outhit))))
                                              (Default|Rotate90 _asbp_tube)))))
                                      (else
                                        (bind _asbp_wires (Utilities|Casting|CastToBP_Wires (.HitActor (Collision|BreakHitResult _outhit)))
                                          (:then
                                            (bind _output_get_3 (Variables|Default|SetAs%20BP%20Wires _asbp_wires))
                                            (bind _assphere_collision (Utilities|Casting|CastToSphereComponent (.HitComponent (Collision|BreakHitResult _outhit))))
                                            (if (== _assphere_collision (Variables|/Game/Blueprints/MiniGames/BP_Wires.BP_Wires_C|GetSphereA _output_get_3))
                                              (bind _asfirst_person_character_5 (Utilities|Casting|CastToFirstPersonCharacter (Game|GetPlayerCharacter 0)))
                                              (Class|PhysicsConstraintComponent|SetConstrainedComponents (Variables|/Game/Blueprints/MiniGames/BP_Wires.BP_Wires_C|GetPhysicsConstraintA _output_get_3) (Variables|/Game/Blueprints/MiniGames/BP_Wires.BP_Wires_C|GetSphereA _output_get_3) "None" (Variables|/Game/FirstPersonBP/Blueprints/FirstPersonCharacter.FirstPersonCharacter_C|GetFocusSphere _asfirst_person_character_5) "None")
                                              (Variables|/Game/FirstPersonBP/Blueprints/FirstPersonCharacter.FirstPersonCharacter_C|SetWiresCatched _asfirst_person_character_5 true)
                                              (Variables|Default|Setsphere (Variables|/Game/Blueprints/MiniGames/BP_Wires.BP_Wires_C|GetSphereA _output_get_3))
                                              (elif (== _assphere_collision (Variables|/Game/Blueprints/MiniGames/BP_Wires.BP_Wires_C|GetSphereB _output_get_3))
                                                (bind _asfirst_person_character_6 (Utilities|Casting|CastToFirstPersonCharacter (Game|GetPlayerCharacter 0)))
                                                (Class|PhysicsConstraintComponent|SetConstrainedComponents (Variables|/Game/Blueprints/MiniGames/BP_Wires.BP_Wires_C|GetPhysicsConstraintB _output_get_3) (Variables|/Game/Blueprints/MiniGames/BP_Wires.BP_Wires_C|GetSphereB _output_get_3) "None" (Variables|/Game/FirstPersonBP/Blueprints/FirstPersonCharacter.FirstPersonCharacter_C|GetFocusSphere _asfirst_person_character_6) "None")
                                                (Variables|/Game/FirstPersonBP/Blueprints/FirstPersonCharacter.FirstPersonCharacter_C|SetWiresCatched _asfirst_person_character_6 true)
                                                (Variables|Default|Setsphere (Variables|/Game/Blueprints/MiniGames/BP_Wires.BP_Wires_C|GetSphereB _output_get_3)))))
                                          (:CastFailed
                                            (goto _label_3)))))))))))))))))))))
    (:Is%20Not%20Valid
      (goto _label))))

(event Custom|MouseWheelScroll
  (params (Axis%20Value :type Integer))
  (bind _asbp_control_table (Utilities|Casting|CastToBP_ControlTable (Variables|Default|GetTargetedScopableObject)))
  (bind _asw_control_table_display (Utilities|Casting|CastToW_ControlTableDisplay (UserInterface|GetWidget (Variables|/Game/SpaceShip/PilotCockpit/BP_ControlTable.BP_ControlTable_C|GetDisplay _asbp_control_table))))
  (Default|ZoomMap (Variables|/Game/SpaceShip/PilotCockpit/W_ControlTableDisplay.W_ControlTableDisplay_C|GetW_WorldMap _asw_control_table_display) (* Axis%20Value (Variables|Default|GetZoomAmount))))

(event Custom|TryLean
  (bind _pickedobject (Variables|Default|GetPickedObject))
  (Utilities|IsValid _pickedobject
    (:Is%20Valid
      (bind _asbp_kettle (Utilities|Casting|CastToBP_Kettle _pickedobject))
      (Variables|Default|SetMouseXOffset 0.0)
      (Default|Leanon _asbp_kettle)
      (bind _asbp_controller (Utilities|Casting|CastToBP_Controller (Game|GetPlayerController 0)))
      (Default|IgnorePlayerInput _asbp_controller)
      (Development|PrintString (Utilities|String|ToString(Float) (Variables|Default|GetMouseXOffset)) true true "(R=1.000000,G=0.077781,B=0.000000,A=1.000000)"))))

(event Custom|StopLean
  (bind _pickedobject (Variables|Default|GetPickedObject))
  (Utilities|IsValid _pickedobject
    (:Is%20Valid
      (bind _asbp_kettle (Utilities|Casting|CastToBP_Kettle _pickedobject))
      (Default|LeanOut _asbp_kettle)
      (bind _asbp_controller (Utilities|Casting|CastToBP_Controller (Game|GetPlayerController 0)))
      (Default|UnignorePlayerInput _asbp_controller))))

(event Custom|OnDialogueIn
  (bind _returnvalue (Game|GetPlayerController 0))
  (bind _dialoguewidget (Variables|Default|GetDialogueWidget))
  (Utilities|IsValid _dialoguewidget
    (:Is%20Valid
      (Widget|SetVisibility _dialoguewidget "Visible")
      (Input|SetIgnoreLookInput _returnvalue true)
      (Input|SetIgnoreMoveInput _returnvalue true)
      (Variables|/Script/Engine.PlayerController|SetbShowMouseCursor _returnvalue true)
      (Variables|Default|SetIsTalking true)
      (Input|SetInputModeUIOnly _returnvalue (Variables|Default|GetDialogueWidget) "DoNotLock"))))

(event Custom|OnDialogueOut
  (bind _returnvalue (Game|GetPlayerController 0))
  (Input|SetIgnoreLookInput _returnvalue false)
  (Input|SetIgnoreMoveInput _returnvalue false)
  (Variables|/Script/Engine.PlayerController|SetbShowMouseCursor _returnvalue false)
  (Variables|Default|SetIsTalking false)
  (Widget|RemovefromParent (Variables|Default|GetDialogueWidget))
  (Input|SetInputModeGameOnly _returnvalue)
  (Default|CallOnDialogueOutDispatcher))

(event Custom|AskForOrder
  (bind _player_camera (Variables|Default|GetPlayer%20Camera))
  (bind _returnvalue (Transformation|GetWorldLocation _player_camera))
  (bind (_outhit _returnvalue_2) (Collision|LineTraceByChannel _returnvalue (+ _returnvalue (* (Math|Vector|GetForwardVector (Variables|Default|GetPlayer%20Camera)) (Variables|Default|GetTraceDistance))) "TraceTypeQuery1" false 0 "None"))
  (if _returnvalue_2
    (bind _asbp_base_passenger (Utilities|Casting|CastToBP_BasePassenger (.HitActor (Collision|BreakHitResult _outhit))))
    (Default|ShowOrder _asbp_base_passenger)))

(event EventBeginPlay
  (Variables|Default|SetPlayer%20Camera (Actor|GetComponentbyClass (Components|GetOwner) "/Script/Engine.CameraComponent")))

(event EventTick
  (params (DeltaSeconds :type Float%20%28single-precision%29))
  (CallFunction|ShowOrderTooltip))

(fn UpdateMouseXOffset
  (params (MouseXDelta :type Float%20%28single-precision%29))
  (Variables|Default|SetMouseXOffset (Math|Float|Clamp(Float) (+ MouseXDelta (Variables|Default|GetMouseXOffset)) -1e+01 0.0)))

(fn OpenDialogueWindow
  (params (DialogueComponent :type Dialogue%20Component%20Object%20Reference))
  (Utilities|IsValid (Variables|Default|GetDialogueWidget)
    (:Is%20Valid
      _)
    (:Is%20Not%20Valid
      (bind _returnvalue (UserInterface|CreateWidget "/Game/Dialogue/UI/W_DialogueWindow.W_DialogueWindow_C"))
      (bind _output_get (Variables|Default|SetDialogueWidget _returnvalue))
      (EventDispatchers|BindEventtoOnDialogueRequestUpdate _output_get (EventDispatchers|CreateEvent :!event NextDialogue))))
  (CallFunction|UpdateDialogueWindow DialogueComponent)
  (UserInterface|Viewport|AddtoViewport (Variables|Default|GetDialogueWidget) 0)
  (return))

(fn NextDialogue
  (params (DialogueComponent :type Dialogue%20Component%20Object%20Reference) (ChoiseIndex :type Integer))
  (bind _returnvalue (Class|DialogueComponent|ChooseDialogueOption DialogueComponent ChoiseIndex))
  (if _returnvalue
    (CallFunction|UpdateDialogueWindow DialogueComponent)
    (else
      (CallFunction|OnDialogueOut))))

(fn UpdateDialogueWindow
  (params (DialogueComponent :type Dialogue%20Component%20Object%20Reference))
  (Utilities|IsValid (Variables|Default|GetDialogueWidget)
    (:Is%20Valid
      (Utilities|Array|Clear (LocalVariables|GetChoiseDate))
      (for _array_element (Class|DialogueComponent|GetDialogueOptions DialogueComponent)
        (bind _returnvalue (Game|ConstructObjectfromClass "/Game/Dialogue/UI/BP_DialogueChoiseData.BP_DialogueChoiseData_C" DialogueComponent))
        (Variables|/Game/Dialogue/UI/BP_DialogueChoiseData.BP_DialogueChoiseData_C|SetChoiseText _returnvalue (.Text (Utilities|Struct|BreakDlgEdge _array_element)))
        (Utilities|Array|Add (LocalVariables|GetChoiseDate) _returnvalue))
      (Default|UpdateDialogue (Variables|Default|GetDialogueWidget) (Utilities|Struct|MakeST_DialogueData DialogueComponent (Class|DialogueComponent|GetSpeakerName DialogueComponent) (Class|DialogueComponent|GetDialogueText DialogueComponent) (LocalVariables|GetChoiseDate)))
      (return))))

(fn GiveObjectHandle
  (params (ObjectToGive :type BP%20Base%20Pickable%20Object%20Object%20Reference) (Reciever :type Object%20Receiver%20Interface))
  (bind _returnvalue (Class|ObjectReceiver|ReceiveObject Reciever ObjectToGive))
  (if _returnvalue
    (CallFunction|DropPickedObject)
    (Actor|DestroyActor ObjectToGive)))

(fn ShowOrderTooltip
  (bind _player_camera (Variables|Default|GetPlayer%20Camera))
  (bind _returnvalue (Transformation|GetWorldLocation _player_camera))
  (bind (_outhit _returnvalue_2) (Collision|LineTraceByChannel _returnvalue (+ _returnvalue (* (Math|Vector|GetForwardVector (Variables|Default|GetPlayer%20Camera)) (Variables|Default|GetTraceDistance))) "TraceTypeQuery1" false 0 "None"))
  (if _returnvalue_2
    (bind _asbp_base_passenger (Utilities|Casting|CastToBP_BasePassenger (.HitActor (Collision|BreakHitResult _outhit)))
      (:then
        (if (and (Variables|/Script/FlightAttendantSim.FABaseCharacter|GetIsSitting _asbp_base_passenger) (Variables|/Game/FoodServing/BP_PassengerOrderComponent.BP_PassengerOrderComponent_C|GetIsOrdered? (Variables|/Game/Characters/BP_BasePassenger.BP_BasePassenger_C|GetOrder%20Component _asbp_base_passenger)))
          (Utilities|IsValid (Variables|Default|GetOrderToolTipWidget)
            (:Is%20Valid
              _)
            (:Is%20Not%20Valid
              (bind _returnvalue_3 (UserInterface|CreateWidget "/Game/FoodServing/UI/W_OrderToolTip.W_OrderToolTip_C" (Game|GetPlayerController 0)))
              (UserInterface|Viewport|AddtoViewport _returnvalue_3 0)
              (Variables|Default|SetOrderToolTipWidget _returnvalue_3)))
          (Widget|SetVisibility (Variables|Default|GetOrderToolTipWidget) "Visible")
          (else
            (Utilities|IsValid (Variables|Default|GetOrderToolTipWidget) :!label _label
              (:Is%20Valid
                (Widget|SetVisibility (Variables|Default|GetOrderToolTipWidget) "Hidden"))))))
      (:CastFailed
        (goto _label)))
    (else
      (goto _label))))