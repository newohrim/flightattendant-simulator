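; BP_PlaneDoor is an interactable door, named as a plane door, that slides open and closed along a path.
; Interact flips IsOpened and plays or reverses the DoorOpening timeline.
; The timeline's LinearAlpha samples a position on LinePath to move the whole actor without sweeping.
; When the timeline finishes with IsOpened set, it fires OnDoorOpened; closing fires no such event.
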(event Custom|OpenDoor
  (bind _linearalpha (Timeline|DoorOpening Play)
    (:Update
      (Transformation|SetActorLocation (Class|FALinePathComponent|GetLocationonLinePath (Variables|Default|GetLinePath) _linearalpha) false false))
    (:Finished
      (if (Variables|Default|GetIsOpened)
        (Default|CallOnDoorOpened)))))

(event Custom|CloseDoor
  (bind _linearalpha (Timeline|DoorOpening Reverse)
    (:Update
      (Transformation|SetActorLocation (Class|FALinePathComponent|GetLocationonLinePath (Variables|Default|GetLinePath) _linearalpha) false false))
    (:Finished
      (if (Variables|Default|GetIsOpened)
        (Default|CallOnDoorOpened)))))

(event EventBeginPlay
  (|CallParentFunction))

(event Collision|EventActorBeginOverlap
  (params (OtherActor :type Actor%20Object%20Reference))
  (|CallParentFunction OtherActor) ; This node is disabled and will not be called.\nDrag off pins to build functionality.
)

(event EventTick
  (params (DeltaSeconds :type Float%20%28single-precision%29))
  (|CallParentFunction DeltaSeconds) ; This node is disabled and will not be called.\nDrag off pins to build functionality.
)

(fn ConstructionScript
  (|CallParentFunction))

(fn Interact
  (params (TracerComponent :type BP%20Camera%20Tracer%20Component%20Object%20Reference))
  (if (Variables|Default|GetIsOpened)
    (Variables|Default|SetIsOpened false)
    (CallFunction|CloseDoor)
    (else
      (Variables|Default|SetIsOpened true)
      (CallFunction|OpenDoor))))