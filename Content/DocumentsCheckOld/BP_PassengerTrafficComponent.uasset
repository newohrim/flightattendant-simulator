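; Passenger traffic component that runs the document-check phase, feeding passengers one by one to the check waypoint for approval or rejection.
; On BeginPlay it builds passengers from game mode data, then shuffles in fakes cloned from real ones with randomly altered passport or ticket fields.
; Each passenger spawns with hidden documents revealed on arrival.
; Approved real passengers walk to their seats, fakes are destroyed, and correct decisions add score.
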(event Custom|OnDocsApproval
  (bind _maingamemode (Variables|Default|GetMainGameMode))
  (Actor|DestroyActor (stale Custom|NextPassenger _returnvalue_2))
  (if (.isfake (Utilities|Array|Get(acopy) (Variables|Default|GetPassengersListWithFakes) (stale Custom|NextPassenger _output_get)))
    (Development|PrintString "FAKE" true true "(R=1.000000,G=0.000000,B=0.000000,A=1.000000)")
    (Actor|DestroyActor (stale Custom|NextPassenger _returnvalue_3) :!label _label)
    (CallFunction|NextPassenger)
    (elif (.ReturnValue (Utilities|Map|Find (Variables|Default|GetTitleToSeatTable) (Class|TicketInfoStruct|GetSeatTitle (.ticketinfo (Utilities|Array|Get(acopy) (Variables|Default|GetPassengersListWithFakes) (stale Custom|NextPassenger _output_get))))))
      (AI|AIMoveTo (stale Custom|NextPassenger _returnvalue_3) (.location (Default|GetMovetoSpot (.Value (Utilities|Map|Find (Variables|Default|GetTitleToSeatTable) (Class|TicketInfoStruct|GetSeatTitle (.ticketinfo (Utilities|Array|Get(acopy) (Variables|Default|GetPassengersListWithFakes) (stale Custom|NextPassenger _output_get)))))))) 0 5.0 false
        (:then
          (Variables|/Game/DocumentsCheckOld/BP_FABaseGameMode.BP_FABaseGameMode_C|SetPlayersScore _maingamemode (+ (Variables|/Game/DocumentsCheckOld/BP_FABaseGameMode.BP_FABaseGameMode_C|GetPlayersScore _maingamemode) 10)))
        (:OnSuccess
          (Development|PrintString "Success")
          (Default|TaketheSeat (stale Custom|NextPassenger _returnvalue_3) (.Value (Utilities|Map|Find (Variables|Default|GetTitleToSeatTable) (Class|TicketInfoStruct|GetSeatTitle (.ticketinfo (Utilities|Array|Get(acopy) (Variables|Default|GetPassengersListWithFakes) (stale Custom|NextPassenger _output_get)))))))
          (CallFunction|NextPassenger))
        (:OnFail
          (Development|PrintString "Fail" true true "(R=1.000000,G=0.121967,B=0.191678,A=1.000000)")))
      (else
        (Development|PrintString "Seat title was unknown")
        (goto _label)))))

(event Custom|OnDocsDisapproval
  (bind _maingamemode (Variables|Default|GetMainGameMode))
  (if (.isfake (Utilities|Array|Get(acopy) (Variables|Default|GetPassengersListWithFakes) (stale Custom|NextPassenger _output_get)))
    (Variables|/Game/DocumentsCheckOld/BP_FABaseGameMode.BP_FABaseGameMode_C|SetPlayersScore _maingamemode (+ (Variables|/Game/DocumentsCheckOld/BP_FABaseGameMode.BP_FABaseGameMode_C|GetPlayersScore _maingamemode) 10))
    (else
      (Development|PrintString "Mistake" true true "(R=1.000000,G=0.018015,B=0.000000,A=1.000000)")))
  (Actor|DestroyActor (stale Custom|NextPassenger _returnvalue_2))
  (Actor|DestroyActor (stale Custom|NextPassenger _returnvalue_3))
  (CallFunction|NextPassenger))

(event Custom|NextPassenger
  (if (< (Variables|Default|GetCurrentPassengerIndex) (- (Variables|Default|GetPassengersCount) 1))
    (bind _output_get (Variables|Default|SetCurrentPassengerIndex (+ (Variables|Default|GetCurrentPassengerIndex) 1)))
    (bind _returnvalue (Game|SpawnActorfromClass "/Game/DocumentsCheckOld/BP_Document.BP_Document_C" (Transformation|GetActorTransform (Variables|SpawnSpots|GetPassport%20Spawn%20Spot)) "AlwaysSpawn" 0 0))
    (Rendering|SetVisibility (Variables|/Game/DocumentsCheckOld/BP_Document.BP_Document_C|GetPassportMesh _returnvalue) false true)
    (Default|UpdateDocsInfoandUI _returnvalue (.passportinfo (Utilities|Array|Get(acopy) (Variables|Default|GetPassengersListWithFakes) _output_get)) (.ticketinfo (Utilities|Array|Get(acopy) (Variables|Default|GetPassengersListWithFakes) _output_get)))
    (bind _returnvalue_2 (Game|SpawnActorfromClass "/Game/DocumentsCheckOld/BP_Ticket.BP_Ticket_C" (Transformation|GetActorTransform (Variables|SpawnSpots|GetTicketSpawnSpot)) "AlwaysSpawn" 0 0))
    (Rendering|SetVisibility (Variables|/Game/DocumentsCheckOld/BP_Ticket.BP_Ticket_C|GetTicketMesh _returnvalue_2) false true)
    (Default|UpdateTicketInfoandUI _returnvalue_2 (.ticketinfo (Utilities|Array|Get(acopy) (Variables|Default|GetPassengersListWithFakes) _output_get)))
    (bind _returnvalue_3 (Game|SpawnActorfromClass "/Game/DocumentsCheckOld/Characters/BP_BasePassengerOld.BP_BasePassengerOld_C" (Transformation|GetActorTransform (Variables|SpawnSpots|GetPassengerSpawnSpot)) "AlwaysSpawn" 0 0))
    (Pawn|SpawnDefaultController _returnvalue_3)
    (Utilities|Array|Add (Variables|Default|GetSpawnedCharacters) _returnvalue_3)
    (Variables|/Script/Engine.CharacterMovementComponent|SetbOrientRotationToMovement (Variables|/Script/Engine.Character|GetCharacterMovement _returnvalue_3) true)
    (AI|AIMoveTo _returnvalue_3 (Transformation|GetActorLocation (Variables|Waypoints|GetPassportCheckWaypoint)) 0 5.0 false
      (:OnSuccess
        (Transformation|SetActorRotation _returnvalue_3 (Transformation|GetActorRotation (Variables|Waypoints|GetPassportCheckWaypoint)))
        (Rendering|SetVisibility (Variables|/Game/DocumentsCheckOld/BP_Document.BP_Document_C|GetPassportMesh _returnvalue) true true)
        (Rendering|SetVisibility (Variables|/Game/DocumentsCheckOld/BP_Ticket.BP_Ticket_C|GetTicketMesh _returnvalue_2) true true)))
    (else
      (Default|DocumentsCheckPhaseCompleted (Variables|Default|GetMainGameMode)))))

(event EventBeginPlay
  (bind _asbp_fabase_game_mode (Utilities|Casting|CastToBP_FABaseGameMode (Game|GetGameMode))
    (:then
      (bind _output_get (Variables|Default|SetMainGameMode _asbp_fabase_game_mode))
      (Variables|/Game/DocumentsCheckOld/BP_FABaseGameMode.BP_FABaseGameMode_C|SetPassengersTrafficManager _output_get self)
      (CallFunction|GeneratePassengersList 6)
      (CallFunction|GeneratePassengerswithFakes (Variables|Default|GetPassengersList))
      (|WaypointsInit))
    (:CastFailed
      (Development|PrintString "Wrong Game Mode!" true true "(R=1.000000,G=0.061979,B=0.091826,A=1.000000)"))))

(fn GeneratePassengersList
  (params (Count :type Integer))
  (Utilities|Array|Resize (Variables|Default|GetPassengersList) Count)
  (for _index (range 0 (- Count 1))
    (Utilities|Array|SetArrayElem (Variables|Default|GetPassengersList) _index (Utilities|Struct|MakeBPS_Passenger false (Utilities|Array|Get(acopy) (Class|FABaseGameMode|GetPassportsList (Variables|Default|GetMainGameMode)) _index) (Utilities|Array|Get(acopy) (Class|FABaseGameMode|GetTicketsList (Variables|Default|GetMainGameMode)) _index)))))

(fn GeneratePassengerswithFakes
  (params (Passengers :type Array%20of%20BPS%20Passenger%20Structures))
  (LocalVariables|SetCount (Utilities|Array|Length Passengers))
  (LocalVariables|SetFakePassengersCount (Math|Random|RandomIntegerinRange (Variables|Default|GetMinFakePassengersCount) (Variables|Default|GetMaxFakePassengersCount)))
  (bind _output_get (Variables|Default|SetPassengersListWithFakes (Variables|Default|GetPassengersList)))
  (Utilities|Array|Resize _output_get (+ (LocalVariables|GetCount) (LocalVariables|GetFakePassengersCount)))
  (for _index (range (LocalVariables|GetCount) (- (+ (LocalVariables|GetCount) (LocalVariables|GetFakePassengersCount)) 1))
    (Utilities|Array|SetArrayElem (Variables|Default|GetPassengersListWithFakes) _index (CallFunction|MakeFakePassenger (Utilities|Array|Get(acopy) (Variables|Default|GetPassengersListWithFakes) (Math|Random|RandomIntegerinRange 0 (- (LocalVariables|GetCount) 1))))))
  (Utilities|Array|Shuffle (Variables|Default|GetPassengersListWithFakes))
  (bind _output_get_2 (Variables|Default|SetPassengersCount (+ (LocalVariables|GetCount) (LocalVariables|GetFakePassengersCount))))
  (bind _asbp_fabase_game_mode (Utilities|Casting|CastToBP_FABaseGameMode (Game|GetGameMode)))
  (Variables|/Game/DocumentsCheckOld/BP_FABaseGameMode.BP_FABaseGameMode_C|SetPlayersMaxScore _asbp_fabase_game_mode (* _output_get_2 10)))

(fn MakeFakePassenger
  (params (Real%20Passenger :type BPS%20Passenger%20Structure%20%28by%20ref%29))
  (bind (_isfake _passportinfo _ticketinfo) (Utilities|Struct|BreakBPS_Passenger Real%20Passenger))
  (bind _returnvalue (Math|Random|RandomIntegerinRange 0 7))
  (bind _alphabet (Variables|Default|GetAlphabet))
  (Utilities|Array|Clear (LocalVariables|GetExcludedIndicies))
  (LocalVariables|SetCurrentCountOfMistakes 0)
  (LocalVariables|SetLoopCompletenessCondition true)
  (bind _asbp_fabase_game_mode (Utilities|Casting|CastToBP_FABaseGameMode (Game|GetGameMode))
    (:then
      (bind _returnvalue_2 (Class|DocsInfoStruct|CopyInstance _passportinfo _passportinfo))
      (bind _returnvalue_3 (Class|TicketInfoStruct|CopyInstance _ticketinfo _ticketinfo))
      (LocalVariables|SetNumOfMistakes (Math|Random|RandomInteger (+ (Variables|Default|GetMaxNumOfMistakesInFake) 1)))
      (while (LocalVariables|GetLoopCompletenessCondition)
        (if (Utilities|Array|ContainsItem (LocalVariables|GetExcludedIndicies) _returnvalue)
          (Development|PrintString "TRUE" true true "(R=1.000000,G=0.000000,B=0.178815,A=1.000000)")
          (else
            (Development|PrintString "PASS" true true "(R=0.040347,G=1.000000,B=0.038727,A=1.000000)")
            (switch int _returnvalue
              (:0
                (Variables|/Script/FlightAttendantSim.DocsInfoStruct|SetLastName _returnvalue_2 (Class|DocsInfoStruct|GetLastName (Class|FABaseGameMode|GetRandomDoc _asbp_fabase_game_mode))))
              (:1
                (Variables|/Script/FlightAttendantSim.DocsInfoStruct|SetFirstName _returnvalue_2 (Class|DocsInfoStruct|GetFirstName (Class|FABaseGameMode|GetRandomDoc _asbp_fabase_game_mode))))
              (:2
                (Variables|/Script/FlightAttendantSim.TicketInfoStruct|SetPassengerId _returnvalue_3 (Variables|/Script/FlightAttendantSim.TicketInfoStruct|GetPassengerId (Class|FABaseGameMode|GetRandomTicket _asbp_fabase_game_mode (Class|TicketInfoStruct|GetSeatTitle _ticketinfo)))))
              (:3
                (Variables|/Script/FlightAttendantSim.TicketInfoStruct|SetLastName _returnvalue_3 (Class|TicketInfoStruct|GetLastName (Class|FABaseGameMode|GetRandomTicket _asbp_fabase_game_mode (Class|TicketInfoStruct|GetSeatTitle _ticketinfo)))))
              (:4
                (Variables|/Script/FlightAttendantSim.TicketInfoStruct|SetSeat _returnvalue_3 (Utilities|String|BuildString(Integer) "" "" (+ (Variables|Default|GetMaxSeatTitleNum) 1) (Utilities|String|GetSubstring _alphabet (Math|Random|RandomIntegerinRange 0 (- (Utilities|String|Len _alphabet) 1))))))
              (:5
                (Variables|/Script/FlightAttendantSim.TicketInfoStruct|SetDepartureDate _returnvalue_3 (Class|DocsInfoStruct|GenerateRandomDate 1950 2020)))
              (:6
                (Variables|/Script/FlightAttendantSim.TicketInfoStruct|SetDepartureTime _returnvalue_3 (Class|DocsInfoStruct|GenerateRandomTime)))
              (:7
                (Variables|/Script/FlightAttendantSim.DocsInfoStruct|SetExpirationDate _returnvalue_2 (Class|DocsInfoStruct|AddDaystoDate (Class|FABaseGameMode|GetFlightDepartureDate (Variables|Default|GetMainGameMode)) (* (+ (Math|Random|RandomInteger 360) 1) -1)))))
            (Utilities|Array|Add (LocalVariables|GetExcludedIndicies) _returnvalue)
            (bind _output_get (LocalVariables|SetCurrentCountOfMistakes (+ (LocalVariables|GetCurrentCountOfMistakes) 1)))
            (if (>= _output_get (LocalVariables|GetNumOfMistakes))
              (LocalVariables|SetLoopCompletenessCondition false)
              (Development|PrintString "FINISHED")
              (return (Utilities|Struct|MakeBPS_Passenger true _returnvalue_2 _returnvalue_3)))))))
    (:CastFailed
      (Development|PrintString "Wrong GameMode!"))))