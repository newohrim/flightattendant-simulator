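; BP_SpaceSkyBox is an actor that sets up the look of a space sky box mesh.
; Its InitMaterial function applies M_SpaceSkyBox to the mesh, then writes the power, scene brightness and star brightness variables into the MC_SpaceSkyBox material parameter collection.
; InitMaterial runs from both the construction script and BeginPlay, so the settings apply on construction and again when play starts.
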(event EventBeginPlay
  (CallFunction|InitMaterial))

(event Collision|EventActorBeginOverlap
  (params (OtherActor :type Actor%20Object%20Reference)))

(event EventTick
  (params (DeltaSeconds :type Float%20%28single-precision%29)))

(fn ConstructionScript
  (CallFunction|InitMaterial))

(fn InitMaterial
  (Rendering|Material|SetMaterial (Variables|Default|GetSkyBoxMesh) 0 "/Game/Enviroment/SkyBox/M_SpaceSkyBox.M_SpaceSkyBox")
  (Rendering|Material|SetScalarParameterValue "/Game/Enviroment/SkyBox/MC_SpaceSkyBox.MC_SpaceSkyBox" "Power" (Variables|Default|GetPower) :!class /Script/Engine.KismetMaterialLibrary)
  (Rendering|Material|SetScalarParameterValue "/Game/Enviroment/SkyBox/MC_SpaceSkyBox.MC_SpaceSkyBox" "SceneBrightness" (Variables|Default|GetSceneBrightness) :!class /Script/Engine.KismetMaterialLibrary)
  (Rendering|Material|SetScalarParameterValue "/Game/Enviroment/SkyBox/MC_SpaceSkyBox.MC_SpaceSkyBox" "StarBrightness" (Variables|Default|GetStarsBrightness) :!class /Script/Engine.KismetMaterialLibrary))