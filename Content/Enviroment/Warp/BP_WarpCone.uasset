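; BP_WarpCone is an environment actor that displays a warp effect on a cone mesh.
; InitMaterial runs from the construction script and BeginPlay, assigning M_WarpCone to the mesh and pushing speed, dissolve, opacity, power and color variables into MC_WarpConeParams.
; Because the values go to a shared Material Parameter Collection rather than a dynamic material instance, they are global, not per actor.
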(event EventBeginPlay
  (CallFunction|InitMaterial))

(event Collision|EventActorBeginOverlap
  (params (OtherActor :type Actor%20Object%20Reference)))

(event EventTick
  (params (DeltaSeconds :type Float%20%28single-precision%29)))

(fn ConstructionScript
  (CallFunction|InitMaterial))

(fn InitMaterial
  (Rendering|Material|SetMaterial (Variables|Default|GetWarpConeMesh) 0 "/Game/Enviroment/Warp/M_WarpCone.M_WarpCone")
  (Rendering|Material|SetScalarParameterValue "/Game/Enviroment/Warp/MC_WarpConeParams.MC_WarpConeParams" "WarpSpeed" (Variables|Default|GetWarpSpeed) :!class /Script/Engine.KismetMaterialLibrary)
  (Rendering|Material|SetScalarParameterValue "/Game/Enviroment/Warp/MC_WarpConeParams.MC_WarpConeParams" "Dissolve" (Variables|Default|GetDissolve) :!class /Script/Engine.KismetMaterialLibrary)
  (Rendering|Material|SetScalarParameterValue "/Game/Enviroment/Warp/MC_WarpConeParams.MC_WarpConeParams" "Opacity" (Variables|Default|GetOpacity) :!class /Script/Engine.KismetMaterialLibrary)
  (Rendering|Material|SetScalarParameterValue "/Game/Enviroment/Warp/MC_WarpConeParams.MC_WarpConeParams" "Power" (Variables|Default|GetPower) :!class /Script/Engine.KismetMaterialLibrary)
  (Rendering|Material|SetVectorParameterValue "/Game/Enviroment/Warp/MC_WarpConeParams.MC_WarpConeParams" "WarpColor" (Variables|Default|GetWarpColor) :!class /Script/Engine.KismetMaterialLibrary))