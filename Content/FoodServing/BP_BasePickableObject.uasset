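; Base Blueprint for pickable objects in the food-serving game, letting them be carried in front of the player camera and dropped.
; Pickup disables mesh physics, gravity and Pawn blocking, and binds to an Update dispatcher fired each Tick; Drop reverses this.
; Carried objects follow camera yaw with clamped lift, auto-dropping if left too far behind.
; Non-swept moves, as on pickup, also update contents when the object is a BP_Tray.
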(event Custom|OnItemDropped
  (bind _objectmesh (Variables|Default|GetObjectMesh))
  (Physics|SetSimulatePhysics _objectmesh true)
  (Collision|SetCollisionResponsetoChannel _objectmesh "ECC_Pawn" "ECR_Block")
  (Physics|SetEnableGravity _objectmesh true))

(event Custom|OnItemPicked
  (bind _objectmesh (Variables|Default|GetObjectMesh))
  (Physics|SetSimulatePhysics _objectmesh false)
  (Collision|SetCollisionResponsetoChannel _objectmesh "ECC_Pawn" "ECR_Ignore")
  (Physics|SetEnableGravity _objectmesh false)
  (CallFunction|UpdateObjectTransform false))

(event EventBeginPlay)

(event Collision|EventActorBeginOverlap
  (params (OtherActor :type Actor%20Object%20Reference)))

(event EventTick
  (params (DeltaSeconds :type Float%20%28single-precision%29))
  (Default|CallUpdate true))

(fn ConstructionScript)

(fn PickUp
  (params (PlayerCamera :type Camera%20Component%20Object%20Reference) (TracerComponent :type BP%20Camera%20Tracer%20Component%20Object%20Reference))
  (if (not (Variables|Default|GetIsPicked?))
    (Variables|Default|SetPlayerCamera PlayerCamera)
    (Variables|Default|SetIsPicked? true)
    (EventDispatchers|BindEventtoUpdate (EventDispatchers|CreateEvent :!event UpdateObjectTransform))
    (CallFunction|OnItemPicked)))

(fn UpdateObjectTransform
  (params (Sweep :type Boolean))
  (bind _playercamera (Variables|Default|GetPlayerCamera))
  (bind _offsetfromcamera (Variables|PickingParams|GetOffsetFromCamera))
  (bind _playercamera_2 (Variables|Default|GetPlayerCamera))
  (bind _returnvalue (Transformation|GetWorldLocation _playercamera_2))
  (bind _returnvalue_2 (Math|Vector|GetForwardVector _playercamera))
  (bind (_x _y) (Math|Vector|BreakVector _returnvalue_2))
  (bind _returnvalue_3 (Math|Vector|MakeVector _x _y 0.0))
  (bind _returnvalue_4 (Math|Vector|Normalize _returnvalue_3))
  (bind _returnvalue_5 (* _returnvalue_4 _offsetfromcamera))
  (bind _returnvalue_6 (+ _returnvalue _returnvalue_5))
  (bind (_x_2 _y_2 _z) (Math|Vector|BreakVector _returnvalue_6))
  (Variables|Default|SetLastTransform (Transformation|GetActorTransform))
  (LocalVariables|SetNewTransform (Math|Transform|MakeTransform (Math|Vector|MakeVector _x_2 _y_2 (+ _z (Math|Float|Clamp(Float) (+ (.Z (Math|Vector|BreakVector (* (Math|Vector|Normalize _returnvalue_2) (Variables|PickingParams|GetOffsetFromCamera)))) (Variables|PickingParams|GetZOffset)) (* -1 (Variables|PickingParams|GetMaxLiftZ)) (Variables|PickingParams|GetMaxLiftZ)))) (Math|Rotator|MakeRotator 0.0 0.0 (.Yaw (Math|Rotator|BreakRotator (Transformation|GetWorldRotation _playercamera_2)))) (Transformation|GetActorScale3D)))
  (if Sweep
    _
    (else
      (bind _asbp_tray (Utilities|Casting|CastToBP_Tray self)
        (:then
          (Default|UpdateContentTransforms _asbp_tray (LocalVariables|GetNewTransform)))
        (:CastFailed
          _))))
  (Transformation|SetActorTransform (LocalVariables|GetNewTransform) Sweep)
  (if (> (Math|Vector|Distance(Vector) (Transformation|GetActorLocation) (Transformation|GetWorldLocation (Variables|Default|GetPlayerCamera))) (* (Variables|PickingParams|GetOffsetFromCamera) 3.0))
    (CallFunction|Drop)))

(fn Drop
  (Variables|Default|SetIsPicked? false)
  (EventDispatchers|UnbindallEventsfromUpdate)
  (CallFunction|OnItemDropped))