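; BP_Cart is a food-serving cart actor that fills itself with trays when play begins.
; On BeginPlay, SpawnTrays loops over the TraysSnapSpots array and spawns a BP_Tray at each spot's location, converted from cart-local to world space.
; Each tray is stored in the Trays array and has physics simulation turned off on its mesh.
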(event EventBeginPlay
  (CallFunction|SpawnTrays))

(event Collision|EventActorBeginOverlap
  (params (OtherActor :type Actor%20Object%20Reference)))

(event EventTick
  (params (DeltaSeconds :type Float%20%28single-precision%29)))

(fn ConstructionScript)

(fn SpawnTrays
  (for _index (range 0 (- (Utilities|Array|Length (Variables|Default|GetTraysSnapSpots)) 1))
    (bind _returnvalue (Game|SpawnActorfromClass "/Game/FoodServing/BP_Tray.BP_Tray_C" (Math|Conversions|ToTransform(Vector) (Math|Transform|TransformLocation (Transformation|GetActorTransform) (.location (Utilities|Array|Get(acopy) (Variables|Default|GetTraysSnapSpots) _index)))) "AlwaysSpawn" 0 0))
    (Utilities|Array|Add (Variables|Default|GetTrays) _returnvalue)
    (Physics|SetSimulatePhysics (Variables|/Game/FoodServing/BP_BasePickableObject.BP_BasePickableObject_C|GetObjectMesh _returnvalue) false)))