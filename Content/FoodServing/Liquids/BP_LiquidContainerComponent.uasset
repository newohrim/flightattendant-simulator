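; BP_LiquidContainerComponent gives its owning actor a fillable liquid volume with a visible surface, for food-serving containers.
; On BeginPlay it spawns a BP_LiquidSurface actor at an owner-relative location and attaches it to the owner.
; AddLiquid clamps the volume to a percentage range, raises or lowers the surface in proportion along the owner's local Z, and hides it when nearly empty.
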(event EventBeginPlay
  (bind _returnvalue (Game|SpawnActorfromClass "/Game/FoodServing/Liquids/BP_LiquidSurface.BP_LiquidSurface_C" (Math|Conversions|ToTransform(Vector) (Math|Transform|TransformLocation (Transformation|GetActorTransform (Components|GetOwner)) (Variables|Default|GetLiquidSurfaceSpawnLoc))) "AlwaysSpawn" 0 0))
  (bind _output_get (Variables|Default|SetLiquidSurface _returnvalue))
  (Transformation|AttachActorToActor _output_get (Components|GetOwner) "None" "KeepRelative" "KeepRelative" "KeepRelative" true))

(fn AddLiquid
  (params (LiquidAmount :type Float%20%28single-precision%29))
  (bind _liquidsurfacespawnloc (Variables|Default|GetLiquidSurfaceSpawnLoc))
  (bind _liquidsurface (Variables|Default|GetLiquidSurface))
  (bind (_x _y _z) (Math|Vector|BreakVector _liquidsurfacespawnloc))
  (bind _defaultsceneroot (Variables|/Game/FoodServing/Liquids/BP_LiquidSurface.BP_LiquidSurface_C|GetDefaultSceneRoot _liquidsurface))
  (bind _output_get (Variables|Default|SetLiquidVolume (Math|Float|Clamp(Float) (+ LiquidAmount (Variables|Default|GetLiquidVolume)) 0.0 1e+02)))
  (Variables|Default|SetLiquidSurfaceHeight (* (/ _output_get 1e+02) (Variables|Default|GetMaxLiquidSurfaceHeight)))
  (Transformation|SetActorLocation (Variables|Default|GetLiquidSurface) (Math|Transform|TransformLocation (Transformation|GetActorTransform (Components|GetOwner)) (Math|Vector|MakeVector _x _y (+ _z (Variables|Default|GetLiquidSurfaceHeight)))) false true)
  (if (< (Variables|Default|GetLiquidVolume) 1.0)
    (Rendering|SetVisibility _defaultsceneroot false true)
    (else
      (Rendering|SetVisibility _defaultsceneroot true true))))