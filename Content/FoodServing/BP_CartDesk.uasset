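; BP_CartDesk is an interactable food-serving cart desk that slides out and back when used.
; BeginPlay derives the starting position from the parent component's relative location plus a fixed offset.
; Interact calls the parent implementation, then toggles Expanded and calls Expand or UnExpand.
; These play or reverse one Timeline, which lerps the actor's relative location along MoveDirection by MoveDistance.
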(event Custom|Expand
  (bind _startrelativepos (Variables|Default|GetStartRelativePos))
  (bind _alpha (Timeline|Timeline Play)
    (:Update
      (Transformation|SetActorRelativeLocation (Math|Vector|Lerp(Vector) _startrelativepos (+ _startrelativepos (* (Variables|Default|GetMoveDirection) (Variables|Default|GetMoveDistance))) _alpha)))))

(event Custom|UnExpand
  (bind _startrelativepos (Variables|Default|GetStartRelativePos))
  (bind _alpha (Timeline|Timeline Reverse)
    (:Update
      (Transformation|SetActorRelativeLocation (Math|Vector|Lerp(Vector) _startrelativepos (+ _startrelativepos (* (Variables|Default|GetMoveDirection) (Variables|Default|GetMoveDistance))) _alpha)))))

(event EventBeginPlay
  (Variables|Default|SetStartRelativePos (+ (.location (Transformation|GetRelativeTransform (Class|Actor|GetParentComponent))) "-30.000000, 0,92.000000")))

(fn ConstructionScript)

(fn Interact
  (params (TracerComponent :type BP%20Camera%20Tracer%20Component%20Object%20Reference))
  (|CallParentFunction TracerComponent)
  (if (Variables|Default|GetExpanded)
    (Variables|Default|SetExpanded false)
    (CallFunction|UnExpand)
    (else
      (Variables|Default|SetExpanded true)
      (CallFunction|Expand))))