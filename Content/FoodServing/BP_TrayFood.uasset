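; BP_TrayFood is a food item for the food-serving part of the game that tracks how heated the meal is.
; Its Heat event adds a delta to MealReadiness, clamped between zero and OverheatTemperature.
; Crossing TargetTemperature or OverheatTemperature triggers BecomeHeated or BecomeOverheated once, guarded by flags that are never cleared here.
; Both state changes only set their flag and print a debug string.
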(event EventBeginPlay
  (|CallParentFunction) ; This node is disabled and will not be called.\nDrag off pins to build functionality.
)

(event Collision|EventActorBeginOverlap
  (params (OtherActor :type Actor%20Object%20Reference))
  (|CallParentFunction OtherActor) ; This node is disabled and will not be called.\nDrag off pins to build functionality.
)

(event EventTick
  (params (DeltaSeconds :type Float%20%28single-precision%29))
  (|CallParentFunction DeltaSeconds) ; This node is disabled and will not be called.\nDrag off pins to build functionality.
)

(event EventHeat
  (params (HeatDelta :type Float%20%28single-precision%29))
  (bind _output_get (Variables|Default|SetMealReadiness (Math|Float|Clamp(Float) (+ HeatDelta (Variables|Default|GetMealReadiness)) 0.0 (Variables|Default|GetOverheatTemperature))))
  (if (>= _output_get (Variables|Default|GetTargetTemperature))
    (if (Variables|Default|GetIsReady)
      _
      (else
        (CallFunction|BecomeHeated)))
    (if (>= (Variables|Default|GetMealReadiness) (Variables|Default|GetOverheatTemperature))
      (if (not (Variables|Default|GetIsOverHeated))
        (CallFunction|BecomeOverheated)))))

(fn ConstructionScript
  (|CallParentFunction))

(fn BecomeHeated
  (Variables|Default|SetIsReady true)
  (Development|PrintString "Heated" true true "(R=0.170019,G=1.000000,B=0.000000,A=1.000000)"))

(fn BecomeOverheated
  (Variables|Default|SetIsOverHeated true)
  (Development|PrintString "Overheated" true true "(R=1.000000,G=0.018907,B=0.000000,A=1.000000)"))