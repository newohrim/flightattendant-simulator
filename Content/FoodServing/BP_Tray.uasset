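; BP_Tray is a pickable food-serving tray that tracks pickable objects resting on it through overlaps with TraySpaceBox.
; UpdateContentTransforms teleports that content to a new tray transform, preserving each item's location and rotation relative to LastTransform.
; While held, the tray's mesh ignores all pickable objects when moving.
; Picking up a stacked tray calls Interact on every BP_CartDesk and clears the stacked flag.
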(event OnComponentBeginOverlap(TraySpaceBox)
  (params (OverlappedComponent :type Primitive%20Component%20Object%20Reference) (OtherActor :type Actor%20Object%20Reference) (OtherComp :type Primitive%20Component%20Object%20Reference) (OtherBodyIndex :type Integer) (bFromSweep :type Boolean) (SweepResult :type Hit%20Result%20Structure%20%28by%20ref%29))
  (bind _asbp_base_pickable_object (Utilities|Casting|CastToBP_BasePickableObject OtherActor))
  (Utilities|Array|Add (Variables|Default|GetTrayContent) _asbp_base_pickable_object))

(event OnComponentEndOverlap(TraySpaceBox)
  (params (OverlappedComponent :type Primitive%20Component%20Object%20Reference) (OtherActor :type Actor%20Object%20Reference) (OtherComp :type Primitive%20Component%20Object%20Reference) (OtherBodyIndex :type Integer))
  (bind _asbp_base_pickable_object (Utilities|Casting|CastToBP_BasePickableObject OtherActor))
  (Utilities|Array|RemoveItem (Variables|Default|GetTrayContent) _asbp_base_pickable_object))

(event EventBeginPlay)

(event Collision|EventActorBeginOverlap
  (params (OtherActor :type Actor%20Object%20Reference)))

(event EventTick
  (params (DeltaSeconds :type Float%20%28single-precision%29))
  (|CallParentFunction 0.0))

(event EventOnItemPicked
  (|CallParentFunction)
  (Collision|ClearMoveIgnoreActors (Variables|Default|GetObjectMesh))
  (bind _outactors (Actor|GetAllActorsOfClass "/Game/FoodServing/BP_BasePickableObject.BP_BasePickableObject_C"))
  (for _array_element _outactors
    (Collision|IgnoreActorwhenMoving (Variables|Default|GetObjectMesh) _array_element true)))

(event EventOnItemDropped
  (|CallParentFunction)
  (Collision|ClearMoveIgnoreActors (Variables|Default|GetObjectMesh)))

(fn ConstructionScript)

(fn PickUp
  (params (PlayerCamera :type Camera%20Component%20Object%20Reference) (TracerComponent :type BP%20Camera%20Tracer%20Component%20Object%20Reference))
  (|CallParentFunction PlayerCamera 0)
  (if (Variables|Default|GetIsStacked?)
    (bind _outactors (Actor|GetAllActorsOfClass "/Game/FoodServing/BP_CartDesk.BP_CartDesk_C"))
    (for _array_element _outactors
      (Default|Interact _array_element)
      (Variables|Default|SetIsStacked? false))))

(fn UpdateContentTransforms
  (params (NewTrayTransform :type Transform))
  (for _array_element (Variables|Default|GetTrayContent)
    (Transformation|SetActorTransform _array_element (Math|Transform|MakeTransform (Math|Transform|TransformLocation NewTrayTransform (.location (Math|Transform|MakeRelativeTransform (Transformation|GetActorTransform _array_element) (Variables|Default|GetLastTransform)))) (Math|Transform|TransformRotation NewTrayTransform (.rotation (Math|Transform|MakeRelativeTransform (Transformation|GetActorTransform _array_element) (Variables|Default|GetLastTransform)))) (Transformation|GetActorScale3D _array_element)) false true)))