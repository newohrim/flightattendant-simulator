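; Component that holds a passenger's food order in the food-serving part of the game.
; MakeOrder flags the passenger as ordered and randomly picks one of three orders drawn from two enum items: both, or either alone.
; ValidateOrder passes when every offered item is in the order, without checking that all ordered items are present.
; CompleteOrder clears the order and flag, then reports the serve to BP_FAGameMode.
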(fn MakeOrder
  (Variables|Default|SetIsOrdered? true)
  (switch int (Math|Random|RandomInteger 3)
    (:0
      (Variables|Default|SetOrder (Utilities|Array|MakeArray "NewEnumerator0" "NewEnumerator1")))
    (:1
      (Variables|Default|SetOrder (Utilities|Array|MakeArray "NewEnumerator0")))
    (:2
      (Variables|Default|SetOrder (Utilities|Array|MakeArray "NewEnumerator1")))))

(fn ValidateOrder
  (params (OrderToValidate :type Array%20of%20E_PassengerOrder%20Enums :default "NewEnumerator0"))
  (for _array_element OrderToValidate
    (if (not (Utilities|Array|ContainsItem (Variables|Default|GetOrder) _array_element))
      (return false)))
  (return true))

(fn CompleteOrder
  (Utilities|Array|Clear (Variables|Default|GetOrder))
  (Variables|Default|SetIsOrdered? false)
  (bind _asbp_fagame_mode (Utilities|Casting|CastToBP_FAGameMode (Game|GetGameMode)))
  (Default|PassengerServed _asbp_fagame_mode))