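; Interactable door for the microwave in food serving, expecting a BP_Microwave as its parent actor.
; Interact toggles Opened, and a timeline lerps relative rotation toward a target computed from the parent component's transform, reversing to close.
; Opening is blocked while the microwave is heating, although Opened still flips.
; Heat and unheat events swap a door material slot between heated and static looks.
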(event Custom|OpenDoor
  (if (not (Variables|/Game/FoodServing/Microwave/BP_Microwave.BP_Microwave_C|GetIsHeating? (Variables|Default|GetMicrowave)))
    (bind _alpha (Timeline|Timeline_0 Play)
      (:Update
        (Transformation|SetActorRelativeRotation (Math|Rotator|Lerp(Rotator) (Variables|Default|GetInitialRotator) (Variables|Default|GetTargetRotator) _alpha))))))

(event Custom|HeatTheDoor
  (Rendering|Material|SetMaterial (Variables|Default|GetDoorMesh) 1 "/Game/FoodServing/Microwave/M_MicrowaveDoorHeated.M_MicrowaveDoorHeated"))

(event Custom|CloseDoor
  (bind _alpha (Timeline|Timeline_0 Reverse)
    (:Update
      (Transformation|SetActorRelativeRotation (Math|Rotator|Lerp(Rotator) (Variables|Default|GetInitialRotator) (Variables|Default|GetTargetRotator) _alpha)))))

(event Custom|UnHeatTheDoor
  (Rendering|Material|SetMaterial (Variables|Default|GetDoorMesh) 1 "/Game/FoodServing/Microwave/M_MicrowaveDoorStatic.M_MicrowaveDoorStatic"))

(event EventBeginPlay
  (bind _returnvalue (Class|Actor|GetParentComponent))
  (bind _returnvalue_2 (Transformation|GetRelativeTransform _returnvalue))
  (Variables|Default|SetInitialRotator (.Rotation (Math|Transform|BreakTransform _returnvalue_2)))
  (Variables|Default|SetTargetRotator (Math|Transform|InverseTransformRotation _returnvalue_2 (Variables|Default|GetTargetRotator)))
  (bind _asbp_microwave (Utilities|Casting|CastToBP_Microwave (Actor|GetParentActor)))
  (Variables|Default|SetMicrowave _asbp_microwave))

(fn ConstructionScript)

(fn Interact
  (params (TracerComponent :type BP%20Camera%20Tracer%20Component%20Object%20Reference))
  (|CallParentFunction TracerComponent)
  (bind _output_get (Variables|Default|SetOpened (not (Variables|Default|GetOpened))))
  (if _output_get
    (CallFunction|OpenDoor)
    (else
      (CallFunction|CloseDoor))))