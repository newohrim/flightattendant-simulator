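; Microwave actor for food serving that heats items inside it, with red and green buttons that only respond while the door is closed.
; Overlaps on an inner box track BPI_Heatable items, while red starts a timed cycle with light and clock widget, and green stops heating and opens the door.
; Tick always fires a heat dispatcher scaled by power and frame time, which is bound on start and unbound on stop.
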(event OnComponentBeginOverlap(InsideContentBox)
  (params (OverlappedComponent :type Primitive%20Component%20Object%20Reference) (OtherActor :type Actor%20Object%20Reference) (OtherComp :type Primitive%20Component%20Object%20Reference) (OtherBodyIndex :type Integer) (bFromSweep :type Boolean) (SweepResult :type Hit%20Result%20Structure%20%28by%20ref%29))
  (bind _asbpi_heatable (Utilities|Casting|CastToBPI_Heatable OtherActor))
  (Utilities|Array|AddUnique (Variables|Default|GetInsideContent) _asbpi_heatable))

(event OnComponentEndOverlap(InsideContentBox)
  (params (OverlappedComponent :type Primitive%20Component%20Object%20Reference) (OtherActor :type Actor%20Object%20Reference) (OtherComp :type Primitive%20Component%20Object%20Reference) (OtherBodyIndex :type Integer))
  (bind _asbpi_heatable (Utilities|Casting|CastToBPI_Heatable OtherActor))
  (Utilities|Array|RemoveItem (Variables|Default|GetInsideContent) _asbpi_heatable))

(event Custom|RedButtonPressed
  (if (not (Variables|/Game/FoodServing/Microwave/BP_MicrowaveDoor.BP_MicrowaveDoor_C|GetOpened (Variables|Default|GetDoor)))
    (if (not (Variables|Default|GetIsHeating?))
      (CallFunction|StartHeating))))

(event Custom|GreenButtonPressed
  (if (not (Variables|/Game/FoodServing/Microwave/BP_MicrowaveDoor.BP_MicrowaveDoor_C|GetOpened (Variables|Default|GetDoor)))
    (if (Variables|Default|GetIsHeating?)
      (CallFunction|StopHeating)
      (Default|OpenDoor (Variables|Default|GetDoor)))))

(event EventBeginPlay
  (bind _asbp_microwave_door (Utilities|Casting|CastToBP_MicrowaveDoor (Variables|/Script/Engine.ChildActorComponent|GetChildActor (Variables|Default|GetDoorActor))))
  (Variables|Default|SetDoor _asbp_microwave_door))

(event EventTick
  (params (DeltaSeconds :type Float%20%28single-precision%29))
  (Default|CallHeatInsideContent (* DeltaSeconds (Variables|Default|GetHeatPower))))

(fn ConstructionScript)

(fn StartHeating
  (Variables|Default|SetIsHeating? true)
  (Rendering|SetVisibility (Variables|Default|GetMicrowaveLight) true false)
  (EventDispatchers|BindEventtoHeatInsideContent (EventDispatchers|CreateEvent :!event HeatContent))
  (bind _returnvalue (Utilities|Time|SetTimerbyFunctionName self "StopHeating" (Variables|Default|GetHeatTimeAmount)))
  (bind _output_get (Variables|Default|SetHeatTimer _returnvalue))
  (bind _asw_microwave_numeric_clock (Utilities|Casting|CastToW_MicrowaveNumericClock (UserInterface|GetUserWidgetObject (Variables|Default|GetNumericClock))))
  (Variables|/Game/FoodServing/Microwave/UI/W_MicrowaveNumericClock.W_MicrowaveNumericClock_C|SetTargetTimer _asw_microwave_numeric_clock _output_get))

(fn StopHeating
  (Variables|Default|SetIsHeating? false)
  (Rendering|SetVisibility (Variables|Default|GetMicrowaveLight) false false)
  (EventDispatchers|UnbindallEventsfromHeatInsideContent))

(fn HeatContent
  (params (HeatAmount :type Float%20%28single-precision%29))
  (for _array_element (Variables|Default|GetInsideContent)
    (Default|Heat _array_element HeatAmount)))