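; BP_Kettle is a pickable kettle that the player tilts to pour liquid.
; While leaning is on, each transform update fires the MakeLean dispatcher, offsetting the kettle sideways and rolling it by the tracer's mouse X offset.
; Past a tilt threshold, a downward trace from the LiquidDispenser socket feeds any hit BP_LiquidContainerComponent, scaled by tilt and frame time, or spawns a decal on other actors.
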(event Custom|LeanOn
  (EventDispatchers|BindEventtoMakeLean (EventDispatchers|CreateEvent :!event Lean))
  (Development|PrintString (Utilities|String|ToString(Float) (Variables|Default|GetLeanProgress))))

(event Custom|LeanOut
  (EventDispatchers|UnbindallEventsfromMakeLean))

(event EventBeginPlay)

(event Collision|EventActorBeginOverlap
  (params (OtherActor :type Actor%20Object%20Reference)))

(event EventTick
  (params (DeltaSeconds :type Float%20%28single-precision%29)))

(event EventOnItemPicked
  (|CallParentFunction)
  (Variables|Default|SetLeanProgress 0.0))

(fn ConstructionScript)

(fn UpdateObjectTransform
  (params (Sweep :type Boolean))
  (|CallParentFunction Sweep)
  (Default|CallMakeLean))

(fn PickUp
  (params (PlayerCamera :type Camera%20Component%20Object%20Reference) (TracerComponent :type BP%20Camera%20Tracer%20Component%20Object%20Reference))
  (|CallParentFunction PlayerCamera TracerComponent)
  (Variables|Default|SetTracerComponent TracerComponent))

(fn Lean
  (bind _playercamera (Variables|Default|GetPlayerCamera))
  (bind _objectmesh (Variables|Default|GetObjectMesh))
  (bind _returnvalue (Transformation|GetSocketLocation _objectmesh "LiquidDispenser"))
  (bind _returnvalue_2 (Transformation|GetWorldRotation _playercamera))
  (Transformation|SetActorLocation (+ (Transformation|GetActorLocation) (Math|Transform|TransformDirection (Transformation|GetActorTransform) (Math|Vector|MakeVector 0.0 (Variables|Default|GetHorizontalOffset) 0.0))) true false)
  (Variables|Default|SetLeanProgress (/ (Variables|/Game/DocumentsCheckOld/BP_CameraTracerComponent.BP_CameraTracerComponent_C|GetMouseXOffset (Variables|Default|GetTracerComponent)) -1e+01))
  (Transformation|SetActorRotation (Math|Interpolation|Ease "Linear" (Variables|Default|GetLeanProgress) (Math|Rotator|MakeRotator 0.0 0.0 (.yaw _returnvalue_2)) (Math|Rotator|MakeRotator (+ (.roll _returnvalue_2) -1.1e+02) 0.0 (.yaw _returnvalue_2)) true))
  (if (> (Variables|Default|GetLeanProgress) 0.35)
    (bind _outhit (Collision|LineTraceByChannel _returnvalue (+ _returnvalue (* (* (Math|Vector|VectorUp) -1.0) (Variables|Default|GetTraceDistance))) "TraceTypeQuery1" false 0 "ForOneFrame"))
    (Utilities|IsValid (.HitActor (Collision|BreakHitResult _outhit))
      (:Is%20Valid
        (Utilities|IsValid (Actor|GetComponentbyClass (.HitActor (Collision|BreakHitResult _outhit)) "/Game/FoodServing/Liquids/BP_LiquidContainerComponent.BP_LiquidContainerComponent_C")
          (:Is%20Valid
            (Default|AddLiquid (Actor|GetComponentbyClass (.HitActor (Collision|BreakHitResult _outhit)) "/Game/FoodServing/Liquids/BP_LiquidContainerComponent.BP_LiquidContainerComponent_C") (* (* (Variables|Default|GetLiquidStreamSpeed) (Utilities|Time|GetWorldDeltaSeconds)) (Variables|Default|GetLeanProgress))))
          (:Is%20Not%20Valid
            (Rendering|Decal|SpawnDecalatLocation "/Game/FoodServing/Materials/Decals/M_BasicDecal.M_BasicDecal" "20.000000,40.000000,40.000000" (.ImpactPoint (Collision|BreakHitResult _outhit)) "-90.000000,0.000000,0.000000" 0.0)))))))