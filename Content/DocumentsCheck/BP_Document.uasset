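; BP_Document is a document actor for the document-check part of the game, showing passport and ticket info through a W_Document widget.
; On BeginPlay it takes the first passport from BP_FABaseGameMode's list, printing a debug message if that entry is invalid.
; UpdateDocsInfoAndUI stores the passport in DocumentsInfoComponent and hands that component, ticket info and itself to the widget.
; It also exposes a camera attach point's world transform.
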(event EventBeginPlay
  (bind _asbp_fabase_game_mode (Utilities|Casting|CastToBP_FABaseGameMode (Game|GetGameMode)))
  (Utilities|IsValid (Utilities|Array|Get(acopy) (Class|FABaseGameMode|GetPassportsList _asbp_fabase_game_mode))
    (:Is%20Valid
      (CallFunction|UpdateDocsInfoandUI (Utilities|Array|Get(acopy) (Class|FABaseGameMode|GetPassportsList _asbp_fabase_game_mode))))
    (:Is%20Not%20Valid
      (Development|PrintString "Doc was None"))))

(event Collision|EventActorBeginOverlap
  (params (OtherActor :type Actor%20Object%20Reference)))

(event EventTick
  (params (DeltaSeconds :type Float%20%28single-precision%29)))

(fn ConstructionScript)

(fn UpdateDocsInfoandUI
  (params (PassportInfo :type Docs%20Info%20Struct%20Object%20Reference) (TicketInfo :type Ticket%20Info%20Struct%20Object%20Reference))
  (Class|FADocumentsInfo|SetDocumentsInfo (Variables|Default|GetDocumentsInfoComponent) PassportInfo)
  (bind _asw_document (Utilities|Casting|CastToW_Document (UserInterface|GetUserWidgetObject (Variables|Default|GetUI_Widget))))
  (Variables|/Game/DocumentsCheck/UI/W_Document.W_Document_C|SetPassportInfo _asw_document (Variables|Default|GetDocumentsInfoComponent))
  (Variables|/Game/DocumentsCheck/UI/W_Document.W_Document_C|SetParentActor _asw_document self)
  (Variables|/Game/DocumentsCheck/UI/W_Document.W_Document_C|SetTicketInfo _asw_document TicketInfo))

(fn GetCameraAttachPoint
  (return (Transformation|GetWorldTransform (Variables|Default|GetCameraAttachPoint))))