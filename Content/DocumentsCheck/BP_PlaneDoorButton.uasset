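; BP_PlaneDoorButton is an interactable button that operates the plane door in the DocumentsCheck area of the game.
; Its Interact override calls the parent, then finds a BP_PlaneDoor with GetActorOfClass and forwards the same TracerComponent to that door's Interact.
; The door is found by class lookup rather than a stored reference, and the event graph holds only disabled default events.
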(event EventBeginPlay
  (|CallParentFunction) ; This node is disabled and will not be called.\nDrag off pins to build functionality.
)

(event Collision|EventActorBeginOverlap
  (params (OtherActor :type Actor%20Object%20Reference))
  (|CallParentFunction OtherActor) ; This node is disabled and will not be called.\nDrag off pins to build functionality.
)

(event EventTick
  (params (DeltaSeconds :type Float%20%28single-precision%29))
  (|CallParentFunction DeltaSeconds) ; This node is disabled and will not be called.\nDrag off pins to build functionality.
)

(fn ConstructionScript
  (|CallParentFunction))

(fn Interact
  (params (TracerComponent :type BP%20Camera%20Tracer%20Component%20Object%20Reference))
  (|CallParentFunction TracerComponent)
  (bind _returnvalue (Actor|GetActorOfClass "/Game/DocumentsCheck/BP_PlaneDoor.BP_PlaneDoor_C"))
  (CallFunction|Interact _returnvalue TracerComponent))