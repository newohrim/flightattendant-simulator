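; BP_FABaseGameMode is the base game mode for a document-check game in which passengers have their papers approved or disapproved.
; Its three functions relay next-passenger, approval and disapproval calls to a PassengersTrafficManager reference, printing a warning when that reference is invalid.
; BeginPlay, Tick and the construction script are empty, and the reference is not assigned in these graphs.
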(event EventBeginPlay)

(event EventTick
  (params (DeltaSeconds :type Float%20%28single-precision%29)))

(fn ConstructionScript)

(fn LetNextPassenger
  (bind _passengerstrafficmanager (Variables|Default|GetPassengersTrafficManager)
    (:then
      (Default|NextPassenger _passengerstrafficmanager))
    (:else
      (Development|PrintString "PassengersTraffic was not set"))))

(fn DocumentApprovedHandler
  (bind _passengerstrafficmanager (Variables|Default|GetPassengersTrafficManager)
    (:then
      (Default|OnDocsApproval _passengerstrafficmanager))
    (:else
      (Development|PrintString "PassengersTraffic was not set"))))

(fn DocumentDisapprovedHandler
  (bind _passengerstrafficmanager (Variables|Default|GetPassengersTrafficManager)
    (:then
      (Default|OnDocsDisapproval _passengerstrafficmanager))
    (:else
      (Development|PrintString "PassengersTraffic was not set"))))