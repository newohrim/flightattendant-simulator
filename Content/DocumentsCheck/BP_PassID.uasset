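; BP_PassID is a passenger ID document in the documents-check gameplay, showing its info through a W_PassIDWidget on its PassWidget component.
; SetDocsInfo copies the supplied document info into that widget, and GetCameraAttachPoint exposes a world transform for camera placement.
; Approve, disapprove and close events report back to the owning passenger through UnShowDocuments, with closing counted the same as disapproval.
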(event Custom|PassengerApproved
  (Class|FABasePassenger|UnShowDocuments (Variables|Default|GetOwningPassenger) true))

(event Custom|PassengerDisapproved
  (Class|FABasePassenger|UnShowDocuments (Variables|Default|GetOwningPassenger) false))

(event Custom|CloseDoc
  (bind _owningpassenger (Variables|Default|GetOwningPassenger))
  (Utilities|IsValid _owningpassenger
    (:Is%20Valid
      (Class|FABasePassenger|UnShowDocuments _owningpassenger false))))

(fn ConstructionScript)

(fn SetDocsInfo
  (params (DocsInfo :type Docs%20Info%20Structure))
  (bind _asw_pass_idwidget (Utilities|Casting|CastToW_PassIDWidget (UserInterface|GetWidget (Variables|Default|GetPassWidget))))
  (Variables|/Game/DocumentsCheck/UI/W_PassIDWidget.W_PassIDWidget_C|SetDocInfo _asw_pass_idwidget DocsInfo))

(fn GetCameraAttachPoint
  (return (Transformation|GetWorldTransform (Variables|Default|GetCameraAttachPoint))))