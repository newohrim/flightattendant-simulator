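; Player component that handles first-person interaction through line traces from the owner's camera.
; Pick traces grab or drop pickables and spawn from dispensers; interact traces toggle cart escorting, trigger interactables or start character dialogue.
; Dialogue locks look and movement, shows the cursor, and fills a reused widget from the speaker's DialogueComponent, advancing by choice.
; It also handles leaning a held kettle with input suppressed and mouse-wheel zoom on control-table maps.
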(event Custom|DropPickedObject
  (bind _pickedobject (Variables|Default|GetPickedObject))
  (Utilities|IsValid _pickedobject
    (:Is%20Valid
      (Default|Drop _pickedobject)
      (Variables|/Script/Engine.CameraComponent|SetbUsePawnControlRotation (Variables|Default|GetPlayer%20Camera) true)
      (bind _asfirst_person_character (Utilities|Casting|CastToFirstPersonCharacter (Components|GetOwner)))
      (Default|OnItemDropped _asfirst_person_character))))

(event Custom|TryPick
  (bind _player_camera (Variables|Default|GetPlayer%20Camera))
  (bind _returnvalue (Transformation|GetWorldLocation _player_camera))
  (Utilities|IsValid (Variables|Default|GetPickedObject)
    (:Is%20Valid
      (if (Variables|/Game/FoodServing/BP_BasePickableObject.BP_BasePickableObject_C|GetIsPicked? (Variables|Default|GetPickedObject))
        (CallFunction|DropPickedObject)
        (else
          (bind (_outhit _returnvalue_2) (Collision|LineTraceByChannel _returnvalue (+ _returnvalue (* (Math|Vector|GetForwardVector (Variables|Default|GetPlayer%20Camera)) (Variables|Default|GetTraceDistance))) "TraceTypeQuery2" false 0 "None" :!label _label))
          (if _returnvalue_2
            (Development|PrintString (Utilities|GetDisplayName (.HitActor (Collision|BreakHitResult _outhit))))
            (bind _asbp_base_pickable_object (Utilities|Casting|CastToBP_BasePickableObject (.HitActor (Collision|BreakHitResult _outhit)))
              (:then
                (Default|PickUp _asbp_base_pickable_object (Variables|Default|GetPlayer%20Camera) self)
                (Variables|Default|SetPickedObject _asbp_base_pickable_object)
                (bind _asfirst_person_character (Utilities|Casting|CastToFirstPersonCharacter (Components|GetOwner)))
                (Default|OnItemPicked _asfirst_person_character))
              (:CastFailed
                (bind _asbp_dispenser (Utilities|Casting|CastToBP_Dispenser (.HitActor (Collision|BreakHitResult _outhit))))
                (Default|CreateInstance _asbp_dispenser self)))))))
    (:Is%20Not%20Valid
      (goto _label))))

(event Custom|TryInteract
  (bind _player_camera (Variables|Default|GetPlayer%20Camera))
  (bind _returnvalue (Transformation|GetWorldLocation _player_camera))
  (Utilities|IsValid (Variables|Default|GetEscortedCart)
    (:Is%20Valid
      (if (Variables|/Game/FoodServing/BP_Cart.BP_Cart_C|GetIsEscorting? (Variables|Default|GetEscortedCart))
        (Default|EscortEnd (Variables|Default|GetEscortedCart))
        (else
          (if (Variables|Default|GetIsTalking) :!label _label
            (CallFunction|OnDialogueOut)
            (else
              (bind (_outhit _returnvalue_2) (Collision|LineTraceByChannel _returnvalue (+ _returnvalue (* (Math|Vector|GetForwardVector (Variables|Default|GetPlayer%20Camera)) (Variables|Default|GetTraceDistance))) "TraceTypeQuery1" false 0 "None"))
              (if _returnvalue_2
                (Development|PrintString (Utilities|GetDisplayName (.HitActor (Collision|BreakHitResult _outhit))))
                (bind _asbp_cart (Utilities|Casting|CastToBP_Cart (.HitActor (Collision|BreakHitResult _outhit)))
                  (:then
                    (bind _asfirst_person_character (Utilities|Casting|CastToFirstPersonCharacter (Components|GetOwner)))
                    (Default|EscortStart _asbp_cart _asfirst_person_character)
                    (Variables|Default|SetEscortedCart _asbp_cart))
                  (:CastFailed
                    (bind _asbp_base_interactable_object (Utilities|Casting|CastToBP_BaseInteractableObject (.HitActor (Collision|BreakHitResult _outhit)))
                      (:then
                        (Default|Interact _asbp_base_interactable_object))
                      (:CastFailed
                        (bind _asfabase_character (Utilities|Casting|CastToFABaseCharacter (.HitActor (Collision|BreakHitResult _outhit))))
                        (if (not (Variables|Default|GetIsTalking))
                          (CallFunction|OnDialoguein)
                          (Utilities|IsValid (Variables|/Script/FlightAttendantSim.DialogueComponent|GetDialogueContext (Variables|/Script/FlightAttendantSim.FABaseCharacter|GetDialogueComponent _asfabase_character))
                            (:Is%20Valid
                              _)
                            (:Is%20Not%20Valid
                              (Class|FABaseCharacter|Talkto _asfabase_character (Components|GetOwner))))
                          (CallFunction|OpenDialogueWindow (Variables|/Script/FlightAttendantSim.FABaseCharacter|GetDialogueComponent _asfabase_character)))))))))))))
    (:Is%20Not%20Valid
      (goto _label))))

(event Custom|MouseWheelScroll
  (params (Axis%20Value :type Integer))
  (bind _asbp_control_table (Utilities|Casting|CastToBP_ControlTable (Variables|Default|GetTargetedScopableObject)))
  (bind _asw_control_table_display (Utilities|Casting|CastToW_ControlTableDisplay (UserInterface|GetWidget (Variables|/Game/SpaceShip/PilotCockpit/BP_ControlTable.BP_ControlTable_C|GetDisplay _asbp_control_table))))
  (Default|ZoomMap (Variables|/Game/SpaceShip/PilotCockpit/W_ControlTableDisplay.W_ControlTableDisplay_C|GetW_WorldMap _asw_control_table_display) (* Axis%20Value (Variables|Default|GetZoomAmount))))

(event Custom|TryLean
  (bind _pickedobject (Variables|Default|GetPickedObject))
  (Utilities|IsValid _pickedobject
    (:Is%20Valid
      (bind _asbp_kettle (Utilities|Casting|CastToBP_Kettle _pickedobject))
      (Variables|Default|SetMouseXOffset 0.0)
      (Default|Leanon _asbp_kettle)
      (bind _asbp_controller (Utilities|Casting|CastToBP_Controller (Game|GetPlayerController 0)))
      (Default|IgnorePlayerInput _asbp_controller)
      (Development|PrintString (Utilities|String|ToString(Float) (Variables|Default|GetMouseXOffset)) true true "(R=1.000000,G=0.077781,B=0.000000,A=1.000000)"))))

(event Custom|StopLean
  (bind _pickedobject (Variables|Default|GetPickedObject))
  (Utilities|IsValid _pickedobject
    (:Is%20Valid
      (bind _asbp_kettle (Utilities|Casting|CastToBP_Kettle _pickedobject))
      (Default|LeanOut _asbp_kettle)
      (bind _asbp_controller (Utilities|Casting|CastToBP_Controller (Game|GetPlayerController 0)))
      (Default|UnignorePlayerInput _asbp_controller))))

(event Custom|OnDialogueIn
  (bind _returnvalue (Game|GetPlayerController 0))
  (Input|SetIgnoreLookInput _returnvalue true)
  (Input|SetIgnoreMoveInput _returnvalue true)
  (Variables|/Script/Engine.PlayerController|SetbShowMouseCursor _returnvalue true)
  (Variables|Default|SetIsTalking true)
  (Input|SetInputModeUIOnly _returnvalue (Variables|Default|GetDialogueWidget) "DoNotLock"))

(event Custom|OnDialogueOut
  (bind _returnvalue (Game|GetPlayerController 0))
  (Input|SetIgnoreLookInput _returnvalue false)
  (Input|SetIgnoreMoveInput _returnvalue false)
  (Variables|/Script/Engine.PlayerController|SetbShowMouseCursor _returnvalue false)
  (Variables|Default|SetIsTalking false)
  (Widget|RemovefromParent (Variables|Default|GetDialogueWidget))
  (Input|SetInputModeGameOnly _returnvalue))

(event EventBeginPlay
  (Variables|Default|SetPlayer%20Camera (Actor|GetComponentbyClass (Components|GetOwner) "/Script/Engine.CameraComponent")))

(fn UpdateMouseXOffset
  (params (MouseXDelta :type Float%20%28single-precision%29))
  (Variables|Default|SetMouseXOffset (Math|Float|Clamp(Float) (+ MouseXDelta (Variables|Default|GetMouseXOffset)) -1e+01 0.0)))

(fn OpenDialogueWindow
  (params (DialogueComponent :type Dialogue%20Component%20Object%20Reference))
  (Utilities|IsValid (Variables|Default|GetDialogueWidget)
    (:Is%20Valid
      _)
    (:Is%20Not%20Valid
      (bind _returnvalue (UserInterface|CreateWidget "/Game/Dialogue/UI/W_DialogueWindow.W_DialogueWindow_C"))
      (bind _output_get (Variables|Default|SetDialogueWidget _returnvalue))
      (EventDispatchers|BindEventtoOnDialogueRequestUpdate _output_get (EventDispatchers|CreateEvent :!event NextDialogue))))
  (CallFunction|UpdateDialogueWindow DialogueComponent)
  (UserInterface|Viewport|AddtoViewport (Variables|Default|GetDialogueWidget) 0)
  (return))

(fn NextDialogue
  (params (DialogueComponent :type Dialogue%20Component%20Object%20Reference) (ChoiseIndex :type Integer))
  (bind _returnvalue (Class|DialogueComponent|ChooseDialogueOption DialogueComponent ChoiseIndex))
  (if _returnvalue
    (CallFunction|UpdateDialogueWindow DialogueComponent)
    (else
      (CallFunction|OnDialogueOut))))

(fn UpdateDialogueWindow
  (params (DialogueComponent :type Dialogue%20Component%20Object%20Reference))
  (Utilities|IsValid (Variables|Default|GetDialogueWidget)
    (:Is%20Valid
      (Utilities|Array|Clear (LocalVariables|GetChoiseDate))
      (for _array_element (Class|DialogueComponent|GetDialogueOptions DialogueComponent)
        (bind _returnvalue (Game|ConstructObjectfromClass "/Game/Dialogue/UI/BP_DialogueChoiseData.BP_DialogueChoiseData_C" DialogueComponent))
        (Variables|/Game/Dialogue/UI/BP_DialogueChoiseData.BP_DialogueChoiseData_C|SetChoiseText _returnvalue (.Text (Utilities|Struct|BreakDlgEdge _array_element)))
        (Utilities|Array|Add (LocalVariables|GetChoiseDate) _returnvalue))
      (Default|UpdateDialogue (Variables|Default|GetDialogueWidget) (Utilities|Struct|MakeST_DialogueData DialogueComponent (Class|DialogueComponent|GetSpeakerName DialogueComponent) (Class|DialogueComponent|GetDialogueText DialogueComponent) (LocalVariables|GetChoiseDate)))
      (return))))